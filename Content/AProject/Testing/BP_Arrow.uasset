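; BP_Arrow is an arrow projectile that damages the BP_Queen boss and disappears on the first thing it overlaps.
; Shoot launches it along local X at the given velocity and enables query-only collision.
; On overlap it deals damage if the target is the Queen, then halts and disables collision in either case.
; A timeline drives a dynamic material's Amount from a point ahead of the arrow, then destroys the actor.
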(event OnComponentBeginOverlap(ArrowColl)
  (params (OverlappedComponent :type Primitive%20Component%20Object%20Reference) (OtherActor :type Actor%20Object%20Reference) (OtherComp :type Primitive%20Component%20Object%20Reference) (OtherBodyIndex :type Integer) (bFromSweep :type Boolean) (SweepResult :type Hit%20Result%20Structure%20%28by%20ref%29))
  (bind _projectilemovement (Variables|Default|GetProjectileMovement))
  (bind _staticmesh (Variables|Default|GetStaticMesh))
  (bind _staticmesh_2 (Variables|Default|GetStaticMesh))
  (bind _projectilemovement_2 (Variables|Default|GetProjectileMovement))
  (bind _asbp_queen (Utilities|Casting|CastToBP_Queen OtherActor)
    (:then
      ;[1 1 1] 보스와 닿았을 때 데미지 작용.
      (Game|Damage|ApplyDamage _asbp_queen 1.0 0 0)
      (Components|Movement|StopMovementImmediately _projectilemovement)
      (Components|Activation|SetActive _projectilemovement false false)
      (Collision|SetCollisionEnabled (Variables|Default|GetArrow%20Coll) "NoCollision")
      (Rendering|Material|SetVectorParameterValue _staticmesh "Location" (Math|Conversions|ToLinearColor(Vector) (+ (Transformation|GetActorLocation) (* (Transformation|GetActorForwardVector) 85.0))) :!class /Script/Engine.MaterialInstanceDynamic)
      (bind _newtrack_0 (Timeline|Timeline_0 PlayFromStart)
        (:Update
          (Rendering|Material|SetScalarParameterValue _staticmesh "Amount" _newtrack_0 :!class /Script/Engine.MaterialInstanceDynamic)
          (Utilities|FlowControl|DoOnce false
            (:Completed
              (Components|DestroyComponent (Variables|Default|GetStaticMesh1)))))
        (:Finished
          (Actor|DestroyActor))))
    (:CastFailed
      ;[1 1 1] 사물과 닿았을 때 사라지기
      (Components|Movement|StopMovementImmediately _projectilemovement_2)
      (Components|Activation|SetActive _projectilemovement_2 false false)
      (Collision|SetCollisionEnabled (Variables|Default|GetArrow%20Coll) "NoCollision")
      (Rendering|Material|SetVectorParameterValue _staticmesh_2 "Location" (Math|Conversions|ToLinearColor(Vector) (+ (Transformation|GetActorLocation) (* (Transformation|GetActorForwardVector) 85.0))) :!class /Script/Engine.MaterialInstanceDynamic)
      (bind _newtrack_0_2 (Timeline|Timeline_1 PlayFromStart)
        (:Update
          (Rendering|Material|SetScalarParameterValue _staticmesh_2 "Amount" _newtrack_0_2 :!class /Script/Engine.MaterialInstanceDynamic)
          (Utilities|FlowControl|DoOnce false
            (:Completed
              (Components|DestroyComponent (Variables|Default|GetStaticMesh1)))))
        (:Finished
          (Actor|DestroyActor))))))

(event Custom|Shoot
  (params (Velocity :type Float%20%28single-precision%29))
  (bind _projectilemovement (Variables|Default|GetProjectileMovement))
  (bind _output_get (Variables|/Script/Engine.ProjectileMovementComponent|SetInitialSpeed _projectilemovement Velocity))
  (Variables|/Script/Engine.ProjectileMovementComponent|SetMaxSpeed _projectilemovement _output_get)
  (Game|Components|ProjectileMovement|SetVelocityinLocalSpace _projectilemovement (Math|Vector|MakeVector Velocity 0.0 0.0))
  (Components|Activation|SetActive (Variables|Default|GetProjectileMovement) true true)
  (Collision|SetCollisionEnabled (Variables|Default|GetArrow%20Coll) "QueryOnly"))

(event EventBeginPlay
  (bind _returnvalue (Rendering|Material|CreateDynamicMaterialInstance (Variables|Debug|GetStaticMeshComponent) 0 0 "None" :!class /Script/Engine.PrimitiveComponent))
  (Variables|Default|SetStaticMesh _returnvalue))

(fn ConstructionScript)