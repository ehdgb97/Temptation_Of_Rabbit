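; Test two-handed bow that AlicePlayer holds in one hand and draws with the other to fire arrows.
; Secondary grab spawns a BP_Arrow on the string, and Tick projects that hand onto the bow axis to move the string within a limit.
; Release plays the SnapBack timeline, detaching and shooting the arrow with draw-scaled force.
; When dropped, the bow eases toward a camera-relative spot on its last-held side, facing the player.
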(event Custom|Shoot
  (Components|Timeline|SetPlayRate (Variables|Default|GetSnapBack) (/ 1.0 0.05))
  (Utilities|FlowControl|Sequence
    (:then_0
      (Audio|PlaySound2D "/Game/AProject/Blueprints/Shhoot.Shhoot" 1.0 1.0 0.0 0 0))
    (:then_1
      (bind _newtrack0 (Timeline|SnapBack PlayFromStart)
        (:Update
          (Transformation|SetRelativeLocation (Variables|Default|GetString) (Math|Vector|Lerp(Vector) (Variables|Default|GetStringRelativeLocation) (Variables|/Script/Engine.SceneComponent|GetRelativeLocation (Variables|Default|GetStringCollision)) _newtrack0) false false)
          (if (> _newtrack0 0.8)
            (bind _arrow (Variables|Default|GetArrow)
              (:then
                (Transformation|DetachFromActor _arrow "KeepWorld" "KeepWorld" "KeepWorld")
                (Default|Shoot (Variables|Default|GetArrow) (Math|Float|MapRangeClamped (Variables|Default|GetForceLength) 0.0 6e+01 0.0 3e+03)))
              (:else))))))))

(event EventSecondaryGrabReleased
  (params (Hand :type Scene%20Component%20Object%20Reference))
  ;[1 1 1] 활을 놓았을 때
  (Variables|Default|SetSecondHand 0)
  (Actor|Tick|SetActorTickEnabled false)
  (CallFunction|Shoot))

(event EventSecondaryGrabPressed
  (params (Hand :type Scene%20Component%20Object%20Reference))
  (Variables|Default|SetSecondHand Hand)
  (Actor|Tick|SetActorTickEnabled true)
  (bind _returnvalue (Game|SpawnActorfromClass "/Game/AProject/Testing/BP_Arrow.BP_Arrow_C" (Math|Transform|MakeTransform "0, 0, 0" "0, 0, 0" "1.200000,2.500000,2.500000") "AlwaysSpawn" 0 0))
  (bind _output_get (Variables|Default|SetArrow _returnvalue))
  (Transformation|AttachComponentToComponent _output_get (Variables|Default|GetString) "None" "SnapToTarget" "SnapToTarget" "KeepWorld" false)
  (Audio|PlaySound2D "/Game/AProject/Blueprints/Loading.Loading" 1.0 1.0 0.0 0 0))

(event EventTick
  (params (DeltaSeconds :type Float%20%28single-precision%29))
  (bind _returnvalue (Transformation|GetActorLocation))
  (bind _returnvalue_2 (Transformation|GetActorLocation))
  (bind _alice (Variables|Default|GetAlice))
  (bind _alice_2 (Variables|Default|GetAlice))
  (bind _camera (Variables|/Game/KGW/VRTemplate/Blueprints/AlicePlayer.AlicePlayer_C|GetCamera _alice))
  (bind _camera_2 (Variables|/Game/KGW/VRTemplate/Blueprints/AlicePlayer.AlicePlayer_C|GetCamera _alice_2))
  (bind _returnvalue_3 (Math|Vector|GetForwardVector _camera))
  (bind _returnvalue_4 (Transformation|GetWorldLocation _camera))
  (bind _returnvalue_5 (Math|Vector|GetForwardVector _camera_2))
  (bind _returnvalue_6 (Transformation|GetWorldLocation _camera_2))
  (bind _returnvalue_7 (- _returnvalue_6 _returnvalue_2))
  (bind _returnvalue_8 (- _returnvalue_4 _returnvalue))
  (Utilities|FlowControl|Sequence
    (:then_0
      (bind _secondhand (Variables|Default|GetSecondHand)
        (:then
          (Variables|Default|SetStringRelativeLocation (Math|Vector|ProjectVectorontoVector (Math|Transform|InverseTransformLocation (Transformation|GetActorTransform) (Transformation|GetWorldLocation _secondhand)) (* (Math|Vector|GetForwardVector (Variables|/Script/Engine.SceneComponent|GetRelativeRotation (Variables|Debug|GetStaticMeshComponent))) -1.0)))
          (Variables|Default|SetForceLength (Math|Vector|VectorLength (- (Variables|Default|GetStringRelativeLocation) (Variables|/Script/Engine.SceneComponent|GetRelativeLocation (Variables|Default|GetStringCollision)))))
          (if (and (< (Math|Vector|DotProduct (Math|Vector|Normalize (- (Variables|Default|GetStringRelativeLocation) (Variables|/Script/Engine.SceneComponent|GetRelativeLocation (Variables|Default|GetStringCollision)))) (* (Math|Vector|GetForwardVector (Variables|/Script/Engine.SceneComponent|GetRelativeRotation (Variables|Debug|GetStaticMeshComponent))) -1.0)) 0.0) (< (Variables|Default|GetForceLength) 6e+01))
            (Transformation|SetRelativeLocation (Variables|Default|GetString) (Variables|Default|GetStringRelativeLocation) false false)))
        (:else)))
    (:then_1
      (if (Variables|Default|GetDroped?)
        (if (Variables|Default|GetIsRighthand)
          (Transformation|SetActorLocationAndRotation (Math|Vector|Lerp(Vector) (Transformation|GetActorLocation) (+ (* (Math|Vector|Normalize (+ (* (Math|Vector|Normalize (+ (* (Math|Vector|Normalize (Math|Vector|MakeVector (.x _returnvalue_5) (.y _returnvalue_5) 0.0)) 2.5) (Math|Vector|GetRightVector _camera_2))) 1.5) (Math|Vector|VectorDown))) 7e+01) _returnvalue_6) 0.15) (Math|Rotator|CombineRotators (Math|Conversions|RotationFromXVector (Math|Vector|Normalize (Math|Vector|MakeVector (.x _returnvalue_7) (.y _returnvalue_7) 0.0))) "0,90.000000, 0"))
          (else
            (Transformation|SetActorLocationAndRotation (Math|Vector|Lerp(Vector) (Transformation|GetActorLocation) (+ (* (Math|Vector|Normalize (+ (* (Math|Vector|Normalize (+ (* (Math|Vector|Normalize (Math|Vector|MakeVector (.x _returnvalue_3) (.y _returnvalue_3) 0.0)) 2.5) (* (Math|Vector|GetRightVector _camera) -1.0))) 1.5) (Math|Vector|VectorDown))) 7e+01) _returnvalue_4) 0.15) (Math|Rotator|CombineRotators (Math|Conversions|RotationFromXVector (Math|Vector|Normalize (Math|Vector|MakeVector (.x _returnvalue_8) (.y _returnvalue_8) 0.0))) "0,90.000000, 0"))))))))

(event EventPick
  (params (Attach%20To :type Scene%20Component%20Object%20Reference))
  (Variables|Default|SetDroped? false)
  (Utilities|FlowControl|Delay 0.15)
  (bind _returnvalue (Actor|GetActorOfClass "/Game/KGW/VRTemplate/Blueprints/AlicePlayer.AlicePlayer_C"))
  (if (== (Variables|/Game/KGW/VRTemplate/Blueprints/AlicePlayer.AlicePlayer_C|GetHeldComponentRight _returnvalue) (Variables|Default|GetTrueGrabComponent))
    (Variables|Default|SetIsRighthand true)
    (Actor|Tick|SetActorTickEnabled false :!label _label)
    (elif (== (Variables|/Game/KGW/VRTemplate/Blueprints/AlicePlayer.AlicePlayer_C|GetHeldComponentLeft _returnvalue) (Variables|Default|GetTrueGrabComponent))
      (Variables|Default|SetIsRighthand false)
      (goto _label))))

(event EventDrop
  (params (Attach%20To :type Scene%20Component%20Object%20Reference))
  (Variables|Default|SetDroped? true)
  (Actor|Tick|SetActorTickEnabled true))

(event EventBeginPlay
  (Actor|Tick|SetActorTickEnabled false)
  (bind _returnvalue (Actor|GetActorOfClass "/Game/KGW/VRTemplate/Blueprints/AlicePlayer.AlicePlayer_C"))
  (Variables|Default|SetAlice _returnvalue))

(fn ConstructionScript)