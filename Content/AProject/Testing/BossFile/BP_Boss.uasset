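; BP_Boss is the boss enemy: it fights the player with four attack patterns and shows a clear widget on death.
; Tick drives cooldowns, randomly picks wave (Pado), rotating Round, aimed Pizza or teleport-slam (Telpo), and limits wave and teleport repeats.
; Patterns advance through timers and DoOnce gates, setting animation flags and spawning attack actors.
; At half health, phase two multiplies attack damage, halves incoming damage and spawns actors at random positions.
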(event Custom|Pizza
  (params (DeltaSeconds :type Float%20%28single-precision%29))
  (bind _returnvalue (Utilities|Time|GetWorldDeltaSeconds))
  ;[1 1 1] 피자
  (Variables|AnimeBool|SetPizzaAni true)
  (Variables|Default|SetPizzaBlendTime (+ (Variables|Default|GetPizzaBlendTime) _returnvalue))
  ;;[1 1 1] 3초 쳐다보기
  (bind _output_get (Variables|Default|SetAttactStart (+ (Variables|Default|GetAttactStart) _returnvalue)))
  (if (> _output_get (Variables|SkillDegi|GetFin%20JangP%20))
    (Utilities|FlowControl|DoOnce false :!label _label
      (:Completed
        (Effects|SpawnEmitteratLocation 0 (Transformation|GetWorldLocation (Variables|Default|GetPizzaFire)) (Transformation|GetActorRotation))
        (Utilities|FlowControl|Delay 0.2)
        (Effects|SpawnEmitteratLocation 0 (Transformation|GetWorldLocation (Variables|Default|GetPizzaFire)) (Transformation|GetActorRotation))
        (Audio|PlaySound2D 0 1.0 1.0 0.0 0 0)
        (Utilities|FlowControl|Delay 0.7)
        ;;[1 1 1] 범위공격 개시
        (Game|SpawnActorfromClass 0 (Transformation|GetActorTransform) "Undefined" 0 0)
        (Game|SpawnActorfromClass 0 (Transformation|GetActorTransform) "Undefined" 0 0)
        (Utilities|FlowControl|Delay 2.5)
        (Utilities|FlowControl|Sequence
          (:then_0
            (Variables|Default|SetAttactStart 0.0))
          (:then_1
            (Variables|Default|SetPattern%20Cool (Variables|CoolTime|GetCoolTimeOfRound))
            (Variables|AnimeBool|SetPizzaAni false))
          (:then_2
            (Variables|Default|SetPizzaBlendTime 0.0))
          (:then_3
            (goto _label Reset)))))
    (else
      ;;[1 1 1] 범위공격 대기
      (CallFunction|WatchTarget)
      (Utilities|FlowControl|DoOnce false :!label _label_2
        (:Completed
          (bind _returnvalue_2 (Audio|SpawnSound2D "/Game/StarterContent/Audio/Fire01.Fire01" 1.0 1.0 0.0 0))
          (Game|SpawnActorfromClass 0 (Transformation|GetActorTransform) "AlwaysSpawn" 0 0)
          (Utilities|FlowControl|Delay 3.5)
          (Components|Activation|ToggleActive _returnvalue_2)
          (goto _label_2 Reset))))))

(event Custom|Telpo
  (params (DeltaSeconds :type Float%20%28single-precision%29))
  (bind _target (Variables|Components|Gettarget))
  (bind _returnvalue (Transformation|GetActorLocation _target))
  ;[1 1 1] 내 위치로 이동
  (Variables|AnimeBool|SetTelpoAnime true)
  (if (Math|Boolean|Equal(Boolean) (Variables|DoOnce|GetTelpoDoOnce) true)
    (Variables|AnimeBool|SetTelpoAnime false)
    ;;[1 1 1] 러프 걸리는 시간+ 대기시간
    (bind _output_get (Variables|Default|SetAttactStart (+ (Utilities|Time|GetWorldDeltaSeconds) (Variables|Default|GetAttactStart))))
    (if (> _output_get (Variables|Default|GetFin%20TelpoAttack))
      (Variables|AnimeBool|SetTelpoDownAni true)
      (Transformation|SetActorLocation (Math|Vector|Lerp(Vector) (Transformation|GetActorLocation) (Variables|Default|GetTelpoLoca) (* (Utilities|Time|GetWorldDeltaSeconds) 15.0)) true false)
      (Utilities|FlowControl|Delay 0.3)
      (Effects|SpawnEmitteratLocation 0 (Transformation|GetActorLocation) "0, 0, 0" "3.000000,3.000000,3.000000")
      (bind _returnvalue_2 (Effects|SpawnEmitteratLocation 0 (+ (Transformation|GetActorLocation) "0, 0,100.000000") "0.000000, 0,180.000000" "3.000000,3.000000,3.000000"))
      ;;[1 1 1] 범위공격 개시
      (Audio|PlaySound2D 0 1.0 1.0 0.0 0 0)
      (Game|SpawnActorfromClass 0 (Math|Conversions|ToTransform(Vector) (Transformation|GetActorLocation)) "AlwaysSpawn" 0 0)
      (Utilities|FlowControl|Sequence
        (:then_0
          (Variables|Default|SetAttactStart 0.0))
        (:then_1
          (Variables|BanRestart|SetReTelpoCool 0.0))
        (:then_2
          (Variables|Default|SetPattern%20Cool (Variables|CoolTime|GetCoolTimeOfTel)))
        (:then_3
          (Variables|DoOnce|SetTelpoDoOnce false)
          (Utilities|FlowControl|Delay 0.7)
          (Variables|AnimeBool|SetTelpoDownAni false))
        (:then_4
          (Utilities|FlowControl|Delay 1.0)
          (Components|DestroyComponent _returnvalue_2)))
      (else
        ;;[1 1 1] 범위공격 대기
        (Utilities|FlowControl|DoOnce false :!label _label
          (:Completed
            (Game|SpawnActorfromClass 0 (Math|Conversions|ToTransform(Vector) (- (Transformation|GetActorLocation) "0, 0,1500.000000")) "Undefined" 0 0)
            (Utilities|FlowControl|Delay 2.0)
            (goto _label Reset)))))
    (else
      (Utilities|FlowControl|Sequence
        (:then_0
          ;;[1 1 1] 텔레포트
          (Utilities|FlowControl|Delay 0.9)
          (Utilities|FlowControl|DoOnce false :!label _label_2
            (:Completed
              (Variables|Default|SetTelpoLoca _returnvalue)
              (Transformation|SetActorLocation (+ _returnvalue "0.000000,0.000000,1500.000000") true false)
              (Variables|DoOnce|SetTelpoDoOnce true)
              (Utilities|FlowControl|Delay 0.2)
              (Utilities|FlowControl|Sequence
                (:then_0
                  (goto _label_2 Reset))
                (:then_1
                  (goto _label_3 Reset))))))
        (:then_1
          (Utilities|FlowControl|DoOnce false :!label _label_3
            (:Completed
              (Audio|PlaySound2D 0 1.0 1.0 0.0 0 0))))))))

(event Custom|PaDo
  (params (DeltaSeconds :type Float%20%28single-precision%29))
  ;[1 1 1] 파도 시스템
  (if (Variables|AnimeBool|GetPadoTelpoOff)
    ;;[1 1 1] Before Attack Telpo
    (Variables|AnimeBool|SetTelpoAnime true)
    (if (Math|Boolean|Equal(Boolean) (Variables|DoOnce|GetTelpoDoOnce) true)
      (Variables|AnimeBool|SetTelpoAnime false)
      ;;;[1 1 1] 러프 걸리는 시간+ 대기시간
      (bind _output_get (Variables|Default|SetAttactStart (+ (Utilities|Time|GetWorldDeltaSeconds) (Variables|Default|GetAttactStart))))
      (if (> _output_get (Variables|Default|GetFin%20TelpoAttack))
        (Variables|AnimeBool|SetRecallAnime true)
        (Transformation|SetActorLocation (Math|Vector|Lerp(Vector) (Transformation|GetActorLocation) "0, 0,196.000000" (* (Utilities|Time|GetWorldDeltaSeconds) 15.0)) true false)
        (Utilities|FlowControl|Sequence
          (:then_0
            (Utilities|FlowControl|Delay 2.0)
            (Variables|AnimeBool|SetRecallAnime false))
          (:then_1
            (Utilities|FlowControl|Delay 2.0)
            (Variables|AnimeBool|SetPadoTelpoOff false))
          (:then_2
            (Utilities|FlowControl|Delay 2.0)
            (Variables|Default|SetAttactStart 0.0))
          (:then_3
            (Utilities|FlowControl|Delay 2.0)
            (Variables|DoOnce|SetTelpoDoOnce false))))
      (else
        ;;;[1 1 1] 텔레포트
        (Utilities|FlowControl|DoOnce false :!label _label
          (:Completed
            (Audio|PlaySound2D 0 1.0 1.0 0.0 0 0)
            (Utilities|FlowControl|Delay 0.9)
            (Transformation|SetActorLocation "0, 0,1500.000000" true false)
            (Transformation|SetActorRotation "0,-180.000000, 0")
            (Variables|DoOnce|SetTelpoDoOnce true)
            (Utilities|FlowControl|Delay 0.2)
            (goto _label Reset)))))
    (else
      ;;[1 1 1] 패턴 나누기
      (bind _output_get_2 (Variables|Default|SetAttactStart (+ (Utilities|Time|GetWorldDeltaSeconds) (Variables|Default|GetAttactStart))))
      (if (> _output_get_2 (Variables|SkillDegi|GetFin%20PaDo))
        (Variables|AnimeBool|SetPadoAni false)
        ;;[1 1 1 0.5] 정한 파도 방향 보내기
        (if (< (Variables|Default|GetSet%20PadoWay) 0.25)
          (Game|SpawnActorfromClass 0 (Variables|PadoWay|GetUpToDown) "AlwaysSpawn" 0 0)
          (elif (< (Variables|Default|GetSet%20PadoWay) 0.5)
            (Game|SpawnActorfromClass 0 (Variables|PadoWay|GetDownToUp) "AlwaysSpawn" 0 0)
            (elif (< (Variables|Default|GetSet%20PadoWay) 0.75)
              (Game|SpawnActorfromClass 0 (Variables|PadoWay|GetRightToLeft) "AlwaysSpawn" 0 0)
              (else
                (Game|SpawnActorfromClass 0 (Variables|PadoWay|GetLeftToRight) "AlwaysSpawn" 0 0)))))
        ;;[1 1 1] 공격초기화/연속사용 방지/ -패턴쿨타임
        (Utilities|FlowControl|Sequence
          (:then_0
            (Variables|Default|SetAttactStart 0.0)
            (Variables|BanRestart|SetRePado%20Cool 0.0)
            (goto _label_2 Reset))
          (:then_1
            (Variables|Default|SetPattern%20Cool (Variables|CoolTime|GetCoolTimeOfPado))
            (Variables|AnimeBool|SetPadoTelpoOff true)
            (Utilities|FlowControl|Delay 7.0)
            (Variables|Default|SetPadoTelpo false)))
        (else
          ;;[1 1 1 0.5] 파도의 방향 정하기
          (Variables|AnimeBool|SetPadoAni true)
          (Variables|Default|SetSet%20PadoWay (Math|Random|RandomFloatinRange 0.0 1.0))
          (Utilities|FlowControl|DoOnce false :!label _label_2
            (:Completed
              (Utilities|FlowControl|Delay 1.0)
              (Audio|PlaySound2D 0 1.0 1.0 0.0 0 0))))))))

(event Custom|Round
  (params (DeltaSeconds :type Float%20%28single-precision%29))
  ;[1 1 1] 장판 즉시
  (Utilities|FlowControl|Sequence
    (:then_0
      ;;[1 1 1] 패턴 나누기
      (Variables|AnimeBool|SetRoundAttackAni true)
      (bind _output_get (Variables|Default|SetAttactStart (+ (Variables|Default|GetAttactStart) DeltaSeconds)))
      (if (> _output_get (Variables|SkillDegi|GetFin%20F_JangP))
        (bind _output_get_2 (Variables|Default|SetTimerOfFJP (+ (Variables|Default|GetTimerOfFJP) (Utilities|Time|GetWorldDeltaSeconds))))
        (if (> _output_get_2 1.9)
          (Utilities|FlowControl|Delay 1.2)
          (Utilities|FlowControl|Sequence
            (:then_0
              (Variables|Default|SetPattern%20Cool (Variables|CoolTime|GetCoolTimeOfPizza))
              (goto _label_2 Reset))
            (:then_1
              (Variables|Default|SetAttactStart 0.0))
            (:then_2
              (Variables|Default|SetTimerOfFJP 0.0))
            (:then_3
              (Variables|Default|SetClock "0,80.000000, 0"))
            (:then_4
              (Variables|AnimeBool|SetRoundAttackAni false))
            (:then_5
              (goto _label Reset)))
          (else
            (Utilities|FlowControl|Delay 0.1)
            (Variables|Default|SetClock (Math|Rotator|CombineRotators (Variables|Default|GetClock) "0.000000,20.000000,0.000000"))
            ;;[1 1 1] 범위공격 개시
            (CallFunction|FJPWay)
            (bind _returnvalue (Game|SpawnActorfromClass 0 (Variables|Default|GetFJP_Rotation) "AlwaysSpawn" 0 0))
            (Game|SpawnActorfromClass 0 (Variables|Default|GetFJP_Rotation) "Undefined" 0 0)
            (Actor|DestroyActor _returnvalue)))
        (else
          ;;[1 1 1] 범위공격 대기
          (Utilities|FlowControl|DoOnce false :!label _label
            (:Completed
              (CallFunction|WatchTarget))))))
    (:then_1
      (Utilities|FlowControl|DoOnce false :!label _label_2
        (:Completed
          (Audio|PlaySound2D 0 1.0 1.0 0.0 0 0))))))

(event Collision|EventActorBeginOverlap
  (params (OtherActor :type Actor%20Object%20Reference))
  (bind _returnvalue (Transformation|GetActorLocation))
  (bind _target (Variables|Components|Gettarget))
  (bind _returnvalue_2 (Transformation|GetActorLocation _target))
  (bind _returnvalue_3 (- _returnvalue_2 _returnvalue))
  ;[1 1 1] 보스와 캐릭터가 겹쳤을 때
  (Utilities|Casting|CastTo OtherActor)
  (Transformation|SetActorLocation (Variables|Components|Gettarget) (+ (* (Math|Vector|Normalize (Math|Vector|MakeVector (.x _returnvalue_3) (.y _returnvalue_3) 0.0)) 1e+01) (Transformation|GetActorLocation (Variables|Components|Gettarget))) false false))

(event EventBeginPlay
  ;[1 1 1] Target 변수를 BP_Player로 정한다.
  ; 보스의 체력을 설정한다.
  (Development|SetHiddeninGame (Variables|Default|Get2Page) true false)
  (Variables|AnimeBool|SetStartAnime true)
  (CallFunction|SetTargetPlayer)
  (Variables|Health|SetBossHealth (Variables|Health|GetMaxHealth))
  (bind _returnvalue (UserInterface|CreateWidget 0))
  (UserInterface|Viewport|AddtoViewport _returnvalue 0)
  (Utilities|FlowControl|Sequence
    (:then_0
      (Utilities|FlowControl|Delay 4.8)
      (Variables|AnimeBool|SetStartAnime false)
      (bind _returnvalue_2 (UserInterface|CreateWidget 0))
      (Variables|Default|SetClear 0 _returnvalue_2))
    (:then_1
      (Utilities|FlowControl|Delay 3.0)
      (Audio|PlaySound2D 0 1.0 1.0 0.0 0 0))))

(event EventTick
  (params (DeltaSeconds :type Float%20%28single-precision%29))
  (bind _returnvalue (Utilities|Time|GetWorldDeltaSeconds))
  (bind _returnvalue_2 (Utilities|Time|GetWorldDeltaSeconds))
  ;[1 1 1] 보스의 행동 패턴
  (bind _returnvalue_3 (Actor|GetActorOfClass 0))
  (Variables|AboutPlayer|SetPlayerHealth (Variables|Default|Gethealth _returnvalue_3))
  (if (== (Variables|Health|GetBossHealth) 0.0)
    ;;[1 1 1] 애니끝
    (Variables|AnimeBool|SetStartAnime false)
    (Variables|AnimeBool|SetTelpoAnime false)
    (Variables|AnimeBool|SetPadoTelpoOff false)
    (Variables|AnimeBool|SetTelpoDownAni false)
    (Variables|AnimeBool|SetRecallAnime false)
    (Variables|AnimeBool|SetPizzaAni false)
    (Variables|AnimeBool|SetRoundAttackAni false)
    (Variables|AnimeBool|SetPadoAni false)
    (Variables|Default|SetDeathAni true)
    (Utilities|FlowControl|Delay 0.2)
    (Utilities|FlowControl|DoOnce false
      (:Completed
        (Utilities|FlowControl|Sequence
          (:then_0
            (Utilities|FlowControl|Delay 2.0)
            (UserInterface|Viewport|AddtoViewport (.Clear (Variables|Default|GetClear)) 0))
          (:then_1
            (Utilities|FlowControl|Delay 1.8)
            (Variables|Default|SetDownAni true)))))
    (else
      ;;[1 1 1] Comment
      (if (!= (Variables|AboutPlayer|GetPlayerHealth) 0.0)
        (Variables|Default|SetClearTime (+ (Variables|Default|GetClearTime) (Utilities|Time|GetWorldDeltaSeconds)))
        (if (> (Variables|Health|GetBossHealth) (/ (Variables|Health|GetMaxHealth) 2.0))
          ;;[1 1 1] 게임오버시 패턴 멈춤
          (bind _returnvalue_4 (Actor|GetActorOfClass 0 :!label _label))
          (Utilities|IsValid _returnvalue_4
            (:Is%20Valid
              ;;[1 1 1] 패턴 연속 사용 방지
              (Variables|BanRestart|SetReTelpoCool (+ (Variables|BanRestart|GetReTelpoCool) _returnvalue_2))
              (Variables|BanRestart|SetRePado%20Cool (+ (Variables|BanRestart|GetRePado%20Cool) _returnvalue_2))
              ;;[1 1 1] 패턴 쿨타임
              (bind _output_get (Variables|Default|SetPattern%20Cool (- (Variables|Default|GetPattern%20Cool) (Utilities|Time|GetWorldDeltaSeconds))))
              (if (> _output_get (Variables|Default|GetPattern%20Start))
                ;;[1 1 1 0.5] 스킬 정하기
                (Variables|Default|SetSelect%20Skill (Math|Random|RandomFloatinRange 0.0 1.0))
                (else
                  ;;[1 1 1 0.5] 스킬 패턴
                  (if (<= (Variables|Default|GetSelect%20Skill) 0.25)
                    ;;;[1 1 1 0.5] n초동안 패턴 재사용 방지 시스템
                    (if (> (Variables|BanRestart|GetRePado%20Cool) 15.0)
                      (Variables|Default|SetPadoTelpo true)
                      (CallFunction|PaDo _returnvalue)
                      (else
                        (Variables|Default|SetPattern%20Cool 0.02)))
                    (elif (<= (Variables|Default|GetSelect%20Skill) 0.5)
                      (CallFunction|Round _returnvalue)
                      (elif (<= (Variables|Default|GetSelect%20Skill) 0.75)
                        (CallFunction|Pizza _returnvalue)
                        (elif (<= (Variables|Default|GetSelect%20Skill) 1.0)
                          (if (> (Variables|BanRestart|GetReTelpoCool) 5.0)
                            (CallFunction|Telpo _returnvalue)
                            (else
                              (Variables|Default|SetPattern%20Cool 0.02)))))))))))
          (else
            (Utilities|FlowControl|Sequence
              (:then_0
                (goto _label))
              (:then_1
                ;;[1 1 1] 데미지 2배
                (Utilities|FlowControl|DoOnce false
                  (:Completed
                    (Audio|PlaySound2D 0 1.0 1.0 0.0 0 0)
                    (Variables|AttackDamage|SetPadoDamage (* (Variables|AttackDamage|GetPadoDamage) (Variables|Default|GetPage2DamageX)))
                    (Variables|AttackDamage|SetRoundDamage (* (Variables|AttackDamage|GetRoundDamage) (Variables|Default|GetPage2DamageX)))
                    (Variables|AttackDamage|SetPizzaDamage (* (Variables|AttackDamage|GetPizzaDamage) (Variables|Default|GetPage2DamageX)))
                    (Variables|AttackDamage|SetTelpoDamage (* (Variables|AttackDamage|GetTelpoDamage) (Variables|Default|GetPage2DamageX)))
                    (Development|SetHiddeninGame (Variables|Default|Get2Page) false false))))
              (:then_2
                (Utilities|FlowControl|Delay 0.1)
                (Game|SpawnActorfromClass 0 (Math|Transform|MakeTransform (Math|Vector|MakeVector (Math|Random|RandomFloatinRange 1.5e+03 -1.5e+03) (Math|Random|RandomFloatinRange 1.3e+03 -1.3e+03) 1e+03) "0, 0, 0" "1,1,1") "Undefined" 0 0)
                (Game|SpawnActorfromClass 0 (Math|Transform|MakeTransform (Math|Vector|MakeVector (Math|Random|RandomFloatinRange 1.5e+03 -1.5e+03) (Math|Random|RandomFloatinRange 1.3e+03 -1.3e+03) 1e+03) "0, 0, 0" "1,1,1") "Undefined" 0 0)))))
        (else
          (Variables|AnimeBool|SetStartAnime false)
          (Variables|AnimeBool|SetTelpoAnime false)
          (Variables|AnimeBool|SetPadoTelpoOff false)
          (Variables|AnimeBool|SetTelpoDownAni false)
          (Variables|AnimeBool|SetRecallAnime false)
          (Variables|AnimeBool|SetPizzaAni false)
          (Variables|AnimeBool|SetRoundAttackAni false)
          (Variables|AnimeBool|SetPadoAni false)
          (Variables|Default|SetPattern%20Cool 2.0)
          (Variables|Default|SetAttactStart 0.0)
          (Variables|Default|SetTimerOfFJP 0.0)
          (Variables|BanRestart|SetRePado%20Cool 0.0)
          (Variables|BanRestart|SetReTelpoCool 0.0)
          (Variables|Default|SetPizzaBlendTime 0.0))))))

(event Game|Damage|EventAnyDamage
  (params (Damage :type Float%20%28single-precision%29) (DamageType :type Damage%20Type%20Object%20Reference) (InstigatedBy :type Controller%20Object%20Reference) (DamageCauser :type Actor%20Object%20Reference))
  (bind _returnvalue (Transformation|GetActorTransform))
  (Audio|PlaySound2D 0 0.2 1.0 0.0 0 0)
  ;[1 1 1] 데미지를 받고 이미지
  (Variables|AttackDamage|SetApplyDamage (Math|Float|Truncate Damage))
  (if (> (Variables|Health|GetBossHealth) (/ (Variables|Health|GetMaxHealth) 2.0))
    _
    (else
      (Variables|AttackDamage|SetApplyDamage (/ (Variables|AttackDamage|GetApplyDamage) 2))))
  (if (> (Variables|Health|GetBossHealth) (Math|Conversions|ToFloat(Integer) (Variables|AttackDamage|GetApplyDamage)))
    _
    (else
      (Variables|AttackDamage|SetApplyDamage (Math|Float|Truncate (Variables|Health|GetBossHealth)))
      (Utilities|FlowControl|DoOnce false
        (:Completed
          (Utilities|FlowControl|DoOnce false
            (:Completed
              (Audio|PlaySound2D 0 1.0 1.0 0.0 0 0)))))))
  (Variables|Health|SetBossHealth (- (Variables|Health|GetBossHealth) (Math|Conversions|ToFloat(Integer) (Variables|AttackDamage|GetApplyDamage))))
  (Game|SpawnActorfromClass 0 (Math|Transform|MakeTransform (Math|Vector|MakeVector (.x (.location _returnvalue)) (.y (.location _returnvalue)) 4.5e+02) "45.000000,135.000000,0.000000" "1,1,1") "Undefined" 0 0)
  (Variables|Default|SetHitani false)
  (Utilities|FlowControl|Delay 0.1)
  (Variables|Default|SetHitani true)
  (Utilities|FlowControl|Delay 0.4)
  (Variables|Default|SetHitani false))

(fn ConstructionScript)

(fn WatchTarget
  ;[1 1 1] 대상이 타겟을 쳐다본다
  (Transformation|SetActorRotation (Math|Rotator|MakeRotator 0.0 0.0 (.yaw (Math|Rotator|FindLookatRotation (Transformation|GetActorLocation) (Transformation|GetActorLocation (Variables|Components|Gettarget)))))))

(fn SetTargetPlayer
  ;[1 1 1] 태어날 때 BP_Player을 찾아서 target에 담고싶다
  (Utilities|IsValid (Variables|Components|Gettarget)
    (:Is%20Not%20Valid
      (bind _returnvalue (Actor|GetActorOfClass 0))
      (Utilities|IsValid _returnvalue
        (:Is%20Valid
          (Variables|Components|Settarget _returnvalue))))))

(fn FJPWay
  (Variables|Default|SetFJP_Rotation (Math|Transform|MakeTransform (Transformation|GetActorLocation) (Math|Rotator|CombineRotators (Variables|Default|GetClock) (Transformation|GetActorRotation)))))

(fn PadoTelposystem
  (Variables|AnimeBool|SetTelpoDownAni true)
  (Transformation|SetActorLocation (Math|Vector|Lerp(Vector) (Transformation|GetActorLocation) "0, 0,196.000000" (* (Utilities|Time|GetWorldDeltaSeconds) 15.0)) true false)
  (Utilities|FlowControl|Sequence))

(fn NewFunction0
  (if (not true)
    (if (not true)
      (if (not true)
        (if true
          _)))))