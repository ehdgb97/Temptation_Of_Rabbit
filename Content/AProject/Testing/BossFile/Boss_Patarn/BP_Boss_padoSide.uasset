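; BP_Boss_padoSide is a boss wave attack that travels along its forward vector at Speed, using a swept move each Tick.
; BeginPlay plays a fire sound, toggles it after five seconds, and reads PadoDamage from an actor found by class.
; An overlap passing a cast enters a DoOnce that subtracts that damage from a class-found actor's Health and teleport-nudges an actor along the wave's direction.
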(event EventBeginPlay
  (Utilities|FlowControl|Sequence
    (:then_0
      (Utilities|FlowControl|DoOnce false
        (:Completed
          (bind _returnvalue (Audio|SpawnSound2D "/Game/StarterContent/Audio/Fire01.Fire01" 1.0 1.0 0.0 0))
          (Utilities|FlowControl|Delay 5.0)
          (Components|Activation|ToggleActive _returnvalue))))
    (:then_1
      (bind _returnvalue_2 (Actor|GetActorOfClass 0))
      (Variables|Default|SetPado%20Damage (Variables|Default|GetPadoDamage _returnvalue_2))
      (Utilities|FlowControl|DoOnce false) ; enters at Reset
    )))

(event Collision|EventActorBeginOverlap
  (params (OtherActor :type Actor%20Object%20Reference))
  (Utilities|Casting|CastTo OtherActor)
  (Utilities|FlowControl|DoOnce false
    (:Completed
      (bind _returnvalue (Actor|GetActorOfClass 0))
      (Variables|Default|Sethealth _returnvalue (- (Variables|Default|Gethealth _returnvalue) (Variables|Default|GetPado%20Damage)))
      (Utilities|FlowControl|DoOnce false
        (:Completed
          (bind _returnvalue_2 (Actor|GetActorOfClass 0))
          (Transformation|SetActorLocation _returnvalue_2 (+ (* (Math|Vector|Normalize (Transformation|GetActorForwardVector)) 1e+02) (Transformation|GetActorLocation _returnvalue_2)) false false))))))

(event EventTick
  (params (DeltaSeconds :type Float%20%28single-precision%29))
  (Transformation|SetActorLocation (+ (Transformation|GetActorLocation) (* (* (Transformation|GetActorForwardVector) (Variables|Default|Getspeed)) DeltaSeconds)) true false))

(fn ConstructionScript)