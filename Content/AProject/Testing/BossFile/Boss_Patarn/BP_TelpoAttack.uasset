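; BP_TelpoAttack is a boss attack actor that deals TelpoDamage when it begins an overlap.
; BeginPlay copies the damage value from an actor found by class lookup.
; On overlap, a second class lookup supplies the actor whose Health is reduced directly, without checking what overlapped.
; Forward movement scaled by Speed and delta time exists but is disconnected, so Tick does nothing.
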(event EventBeginPlay
  (bind _returnvalue (Actor|GetActorOfClass 0))
  (Variables|Default|SetTelpo%20Damage (Variables|Default|GetTelpoDamage _returnvalue)))

(event Collision|EventActorBeginOverlap
  (params (OtherActor :type Actor%20Object%20Reference))
  (bind _returnvalue (Actor|GetActorOfClass 0))
  (Variables|Default|Sethealth _returnvalue (- (Variables|Default|Gethealth _returnvalue) (Variables|Default|GetTelpo%20Damage))))

(event EventTick
  (params (DeltaSeconds :type Float%20%28single-precision%29))
  ;[1 1 1] P = P0 + GetActorForward * speed * deltaSeconds
)

(fn ConstructionScript)