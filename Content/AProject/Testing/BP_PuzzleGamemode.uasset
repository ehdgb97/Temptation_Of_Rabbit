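; Game mode for a puzzle level that tracks puzzle start, puzzle completion and boss death.
; On BeginPlay it fades in, plays Castle music and caches the stair and switch actors.
; Events switch to Boss music, stop that music, or destroy the three switches.
; BossDied clears AlicePlayer's turn, size and teleport conditions, fades out, then sets its flag after the delay.
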(event Custom|Puzzle%20Start
  (Variables|Default|SetPuzzleStart true))

(event Custom|BossDied
  (bind _returnvalue (Actor|GetActorOfClass "/Game/KGW/VRTemplate/Blueprints/AlicePlayer.AlicePlayer_C"))
  (Variables|/Game/KGW/VRTemplate/Blueprints/AlicePlayer.AlicePlayer_C|SetTurn%20cond _returnvalue false)
  (Variables|/Game/KGW/VRTemplate/Blueprints/AlicePlayer.AlicePlayer_C|SetbSizeCond _returnvalue false)
  (Variables|/Game/KGW/VRTemplate/Blueprints/AlicePlayer.AlicePlayer_C|SetTeleportCond _returnvalue false)
  (CameraFades|StartCameraFade :self (Game|GetPlayerCameraManager 0) :ToAlpha 1.0 :Duration 4.0 :bShouldFadeAudio true :bHoldWhenFinished true)
  (Utilities|FlowControl|Delay 4.0)
  (Variables|Default|SetbBossDied true))

(event Custom|Puzzle%20Finished
  (Variables|Default|SetPuzzleEnd true))

(event Custom|Destory%20Music%202
  (Components|DestroyComponent (stale Custom|DestroyMusic _returnvalue)))

(event Custom|DestroyMusic
  (Components|DestroyComponent (stale EventBeginPlay _returnvalue))
  (bind _returnvalue (Audio|SpawnSound2D "/Game/AProject/BGM/Boss.Boss" 1.0 1.0 0.0 0 false false)))

(event Custom|Switch%20hidden
  (Actor|DestroyActor (Variables|Default|GetSwitchC)))

(event EventBeginPlay
  (CameraFades|StartCameraFade :self (Game|GetPlayerCameraManager 0) :FromAlpha 1.0 :Duration 3.0 :bShouldFadeAudio true :bHoldWhenFinished true)
  (bind _returnvalue (Audio|SpawnSound2D "/Game/AProject/BGM/Castle.Castle" 1.0 1.0 0.0 0 false false))
  (bind _returnvalue_2 (Actor|GetActorOfClass "/Game/AProject/Blueprints/BP_StairA.BP_StairA_C"))
  (bind _returnvalue_3 (Actor|GetActorOfClass "/Game/AProject/Blueprints/BP_StairB.BP_StairB_C"))
  (bind _returnvalue_4 (Actor|GetActorOfClass "/Game/AProject/Blueprints/BP_StairC.BP_StairC_C"))
  (bind _returnvalue_5 (Actor|GetActorOfClass "/Game/AProject/Blueprints/BP_StairD.BP_StairD_C"))
  (bind _returnvalue_6 (Actor|GetActorOfClass "/Game/AProject/Testing/BP_SwitchA.BP_SwitchA_C"))
  (bind _returnvalue_7 (Actor|GetActorOfClass "/Game/AProject/Testing/BP_SwitchB.BP_SwitchB_C"))
  (bind _returnvalue_8 (Actor|GetActorOfClass "/Game/AProject/Testing/BP_SwitchC.BP_SwitchC_C"))
  (Variables|Default|SetSwitchC _returnvalue_8)
  (Variables|Default|SetSwitchB _returnvalue_7)
  (Variables|Default|SetSwitch%20A _returnvalue_6)
  (Variables|Default|Setstair%20D _returnvalue_5)
  (Variables|Default|Setstair%20C _returnvalue_4)
  (Variables|Default|Setstair%20B _returnvalue_3)
  (Variables|Default|SetStairA _returnvalue_2))

(event EventTick
  (params (DeltaSeconds :type Float%20%28single-precision%29)))

(fn ConstructionScript)