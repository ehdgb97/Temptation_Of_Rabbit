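; BP_Enemy is a target that BP_Arrow destroys, awarding more score to BP_EnemySpawner the sooner it is hit after spawning.
; A hit disables collision and drives a dynamic material's Location and Amount through a timeline, adding score and audio before destruction.
; When the spawner's enemy count empties, the hit moves SpawnTimer closer to SpawnReady.
; Tick tracks lifetime and, once the spawner's Second runs out, plays a similar scoreless removal.
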(event OnComponentBeginOverlap(Cube)
  (params (OverlappedComponent :type Primitive%20Component%20Object%20Reference) (OtherActor :type Actor%20Object%20Reference) (OtherComp :type Primitive%20Component%20Object%20Reference) (OtherBodyIndex :type Integer) (bFromSweep :type Boolean) (SweepResult :type Hit%20Result%20Structure%20%28by%20ref%29))
  (bind _bp_enemyspawn (Variables|Default|GetBP_EnemySpawn))
  (bind _bp_enemyspawn_2 (Variables|Default|GetBP_EnemySpawn))
  (bind _bp_enemyspawn_3 (Variables|Default|GetBP_EnemySpawn))
  (Utilities|Casting|CastToBP_Arrow OtherActor)
  (Variables|/Game/AProject/Blueprints/BP_EnemySpawner.BP_EnemySpawner_C|SetCount%20enemy _bp_enemyspawn_2 (- (Variables|/Game/AProject/Blueprints/BP_EnemySpawner.BP_EnemySpawner_C|GetCount%20enemy _bp_enemyspawn_2) 1))
  ;[1 1 1] Set Score
  (if (< (Variables|Default|GetSpawnedTime) 1.5)
    (Variables|Default|SetAddScore 60)
    (elif (< (Variables|Default|GetSpawnedTime) 2.0)
      (Variables|Default|SetAddScore 50)
      (elif (< (Variables|Default|GetSpawnedTime) 2.5)
        (Variables|Default|SetAddScore 40)
        (elif (< (Variables|Default|GetSpawnedTime) 3.5)
          (Variables|Default|SetAddScore 30)
          (elif (< (Variables|Default|GetSpawnedTime) 4.0)
            (Variables|Default|SetAddScore 20)
            (else
              (Variables|Default|SetAddScore 10)))))))
  (Utilities|FlowControl|Sequence
    (:then_0
      ;[1 1 1] Material
      (Rendering|Material|SetVectorParameterValue (Variables|Default|GetNewVar_0) "Location" (Math|Conversions|ToLinearColor(Vector) (Transformation|GetWorldLocation OtherComp)) :!class /Script/Engine.MaterialInstanceDynamic)
      (Collision|SetCollisionEnabled (Variables|Default|GetCube) "NoCollision")
      (bind _newtrack_0 (Timeline|Timeline_0 PlayFromStart)
        (:Update
          (Rendering|Material|SetScalarParameterValue (Variables|Default|GetNewVar_0) "Amount" _newtrack_0 :!class /Script/Engine.MaterialInstanceDynamic)
          (Utilities|FlowControl|DoOnce false
            (:Completed
              (Variables|/Game/AProject/Blueprints/BP_EnemySpawner.BP_EnemySpawner_C|SetScore _bp_enemyspawn_3 (+ (Variables|/Game/AProject/Blueprints/BP_EnemySpawner.BP_EnemySpawner_C|GetScore _bp_enemyspawn_3) (Variables|Default|GetAddScore)))
              (AddComponent|AddAudioComponent false))))
        (:Finished
          (Actor|DestroyActor))))
    (:then_1
      (if (<= (Variables|/Game/AProject/Blueprints/BP_EnemySpawner.BP_EnemySpawner_C|GetCount%20enemy _bp_enemyspawn) 0)
        (Variables|/Game/AProject/Blueprints/BP_EnemySpawner.BP_EnemySpawner_C|SetSpawnTimer _bp_enemyspawn (- (Variables|/Game/AProject/Blueprints/BP_EnemySpawner.BP_EnemySpawner_C|GetSpawnReady _bp_enemyspawn) (/ (- (Variables|/Game/AProject/Blueprints/BP_EnemySpawner.BP_EnemySpawner_C|GetSpawnReady _bp_enemyspawn) (Variables|/Game/AProject/Blueprints/BP_EnemySpawner.BP_EnemySpawner_C|GetSpawnTimer _bp_enemyspawn)) 5.0)))))))

(event EventBeginPlay
  (bind _returnvalue (Rendering|Material|CreateDynamicMaterialInstance (Variables|Default|GetCube) 0 0 "None" :!class /Script/Engine.PrimitiveComponent))
  (Variables|Default|SetNewVar_0 _returnvalue)
  (bind _returnvalue_2 (Actor|GetActorOfClass "/Game/AProject/Blueprints/BP_EnemySpawner.BP_EnemySpawner_C"))
  (Variables|Default|SetBP_EnemySpawn _returnvalue_2))

(event EventTick
  (params (DeltaSeconds :type Float%20%28single-precision%29))
  (bind _bp_enemyspawn (Variables|Default|GetBP_EnemySpawn))
  (if (> (Variables|/Game/AProject/Blueprints/BP_EnemySpawner.BP_EnemySpawner_C|GetSecond _bp_enemyspawn) 0)
    (Variables|Default|SetSpawnedTime (+ (Variables|Default|GetSpawnedTime) (Utilities|Time|GetWorldDeltaSeconds)))
    (else
      (Variables|/Game/AProject/Blueprints/BP_EnemySpawner.BP_EnemySpawner_C|SetCount%20enemy _bp_enemyspawn 0)
      ;[1 1 1] Material
      (Rendering|Material|SetVectorParameterValue (Variables|Default|GetNewVar_0) "Location" (Math|Conversions|ToLinearColor(Vector) (+ (Transformation|GetActorLocation) "0, 0,30.000000")) :!class /Script/Engine.MaterialInstanceDynamic)
      (Collision|SetCollisionEnabled (Variables|Default|GetCube) "NoCollision")
      (Utilities|FlowControl|DoOnce false
        (:Completed
          (bind _newtrack_0 (Timeline|Timeline_1 PlayFromStart)
            (:Update
              (Rendering|Material|SetScalarParameterValue (Variables|Default|GetNewVar_0) "Amount" _newtrack_0 :!class /Script/Engine.MaterialInstanceDynamic)
              (Utilities|FlowControl|DoOnce false
                (:Completed
                  (AddComponent|AddAudioComponent false))))
            (:Finished
              (Actor|DestroyActor))))))))

(fn ConstructionScript)