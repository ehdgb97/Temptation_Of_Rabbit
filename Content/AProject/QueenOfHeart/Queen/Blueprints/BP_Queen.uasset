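; Queen boss that cycles through Shield, Idle, Attack and Rest states on Tick, with DoOnce gates limiting repeat entry.
; Timelines scale a spawned BP_Shield up and down around a volley of randomly angled BP_BossProjectile shots.
; Dropping the shield opens a one-hit damage window; a hit restores the shield or, at zero health, triggers death and notifies BP_PuzzleGamemode.
; Chained voice lines announce shield and attack phases.
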(event Custom|Attack
  (bind _returnvalue (Transformation|GetActorRotation))
  ;[0.1441 0 0 1 45] Attack State
  (Utilities|FlowControl|Sequence
    (:then_0
      ;;[0 0 0 0.5] 공격 준비 블랜딩타임
      (bind _output_get (Variables|Default|SetAttack_Blend_Time (+ (Variables|Default|GetAttack_Blend_Time) (Utilities|Time|GetWorldDeltaSeconds))))
      (if (> _output_get (Variables|Default|GetAttackStart))
        ;;[0 0 0 0.5] 발사횟수
        (if (== (Variables|Default|GetFireTime) 15)
          (Utilities|FlowControl|DoOnce true :!label _label
            (:Completed
              (Utilities|FlowControl|Delay 1.15)
              (Variables|Animate|Bool|SetbAttack_Ani false)
              (Utilities|FlowControl|Delay 3.0)
              (Variables|Default|SetBoss_State "NewEnumerator3")
              (Variables|Default|SetAttack_Blend_Time 0.0)
              (goto _label_2 Reset)))
          (else
            (Game|SpawnActorfromClass "/Game/AProject/QueenOfHeart/QueenSkill/Blueprints/BP_BossProjectile.BP_BossProjectile_C" (Math|Transform|MakeTransform (+ (Transformation|GetWorldLocation (Variables|Default|GetScene)) "0, 0,10.000000") (Math|Rotator|MakeRotator (.roll _returnvalue) (Math|Random|RandomFloatinRange -2e+01 7e+01) (+ (.yaw _returnvalue) (Math|Random|RandomFloatinRange -45.0 45.0))) "1.000000,1.000000,2.000000") "AlwaysSpawn" 0 0)
            (Variables|Default|SetFireTime (+ (Variables|Default|GetFireTime) 1))
            (goto _label Reset)))))
    (:then_1
      (Utilities|FlowControl|DoOnce false :!label _label_2
        (:Completed
          (Variables|Animate|Bool|SetbAttack_Ani true))))))

(event Custom|Rest
  (bind _shieldactor (Variables|Default|GetShieldActor))
  ;[0.05951 0 0 1 45] Rest State
  (bind _새_트랙_0 (Timeline|타임라인_1 ReverseFromEnd)
    (:Update
      (Transformation|SetActorTransform _shieldactor (Math|Transform|MakeTransform (Transformation|GetActorLocation _shieldactor) (.rotation (Transformation|GetActorTransform)) (Math|Vector|MakeVector _새_트랙_0 _새_트랙_0 _새_트랙_0))))
    (:Finished
      (CallFunction|CanDamage)
      (bind _returnvalue (Audio|SpawnSound2D "/Game/AProject/Desa/audio_35_보호막이_풀렸어_.audio_35_보호막이_풀렸어_" 1.0 1.0 0.0 0))
      (EventDispatchers|BindEventtoOnAudioFinished _returnvalue (delegate Custom|Destory%20Sound)))))

(event Custom|Idle
  ;[0.3515 0 0 1 45] Idle State
  ;;[1 1 1] First Meet
  (if (Variables|Default|GetbIs_First_Meeting)
    (Utilities|FlowControl|DoOnce false
      (:Completed
        (Variables|Animate|Bool|SetbFirstMeet_Ani true)
        (Utilities|FlowControl|Delay 0.2)
        (Variables|Animate|Bool|SetbFirstMeet_Ani false)
        (Rendering|SetVisibility (Variables|Default|GetWidget) true false)
        (Utilities|FlowControl|Delay 0.2)
        (Variables|Default|SetBoss_State "NewEnumerator0")
        (Variables|Default|SetbIs_First_Meeting false)))
    (else
      (Utilities|FlowControl|DoOnce true
        (:Completed
          (Utilities|FlowControl|Delay 2.0)
          (Variables|Default|SetBoss_State "NewEnumerator2")
          (bind _returnvalue (Audio|SpawnSound2D "/Game/AProject/Desa/audio_33_여왕이_공격을_한다_.audio_33_여왕이_공격을_한다_" 1.0 1.0 0.0 0))
          (EventDispatchers|BindEventtoOnAudioFinished _returnvalue (delegate Custom|Attack%20Begin)))))))

(event Custom|CanDamage
  ;[0.02416 0 0 1 45] Damaged When Rest State
  (Utilities|FlowControl|DoOnce true) ; enters at Reset
)

(event Custom|Shield
  (bind _shieldactor (Variables|Default|GetShieldActor))
  ;[1 0 0 1 45] Shield State
  (Variables|Animate|Bool|SetbSpawn_Shield_Ani true)
  (bind _returnvalue (AddComponent|AddAudioComponent false))
  (bind _새_트랙_0 (Timeline|타임라인_0 PlayFromStart)
    (:Update
      (Transformation|SetActorTransform _shieldactor (Math|Transform|MakeTransform (Transformation|GetActorLocation _shieldactor) "0, 0, 0" (Math|Vector|MakeVector _새_트랙_0 _새_트랙_0 _새_트랙_0)))
      (Utilities|FlowControl|DoOnce false :!label _label
        (:Completed
          (bind _returnvalue_2 (Audio|SpawnSound2D "/Game/AProject/Desa/audio_31_여왕이_보호막을_썼어____.audio_31_여왕이_보호막을_썼어____" 1.0 1.0 0.0 0))
          (EventDispatchers|BindEventtoOnAudioFinished _returnvalue_2 (delegate Custom|커스텀이벤트_0)))))
    (:Finished
      (Variables|Animate|Bool|SetbSpawn_Shield_Ani false)
      (Components|DestroyComponent _returnvalue)
      (Variables|Default|SetFireTime 0)
      (Variables|Default|SetBoss_State "NewEnumerator1")
      (Utilities|FlowControl|Sequence
        (:then_0
          (goto _label Reset))
        (:then_1
          ;[0.3515 0 0 1 45] Idle State
          (Utilities|FlowControl|DoOnce true) ; enters at Reset
        )))))

(event Custom|Died
  ;[0 0 0 1 45] Died State
  (Variables|Default|SetbDied_Ani true)
  (bind _asbp_puzzle_gamemode (Utilities|Casting|CastToBP_PuzzleGamemode (Game|GetGameMode)))
  (Utilities|FlowControl|Delay 4.0)
  (Default|BossDied _asbp_puzzle_gamemode))

(event Custom|Destory%20Sound%20Shield
  ;[0.05951 0 0 1 45] Rest State
  (Components|DestroyComponent (stale Custom|Destory%20Sound _returnvalue)))

(event Custom|Destory%20Sound
  ;[0.05951 0 0 1 45] Rest State
  (Components|DestroyComponent (stale Custom|Rest _returnvalue))
  (bind _returnvalue (Audio|SpawnSound2D "/Game/AProject/Desa/audio_36_어서_공격해_.audio_36_어서_공격해_" 1.0 1.0 0.0 0))
  (EventDispatchers|BindEventtoOnAudioFinished _returnvalue (delegate Custom|Destory%20Sound%20Shield)))

(event Custom|Attack%20Begin
  ;[0.3515 0 0 1 45] Idle State
  (Audio|SpawnSound2D "/Game/AProject/Desa/audio_34_어서_피해_.audio_34_어서_피해_" 1.0 1.0 0.0 0))

(event Custom|커스텀이벤트_0
  ;[1 0 0 1 45] Shield State
  (Audio|SpawnSound2D "/Game/AProject/Desa/audio_32_지금은_공격이_통하지_않아_.audio_32_지금은_공격이_통하지_않아_" 1.0 1.0 0.0 0))

(event EventBeginPlay
  ;[0 0 0 0.5 30] Begin Play
  (Variables|Default|SetHealth (Variables|Default|GetMax_HP))
  (Variables|Default|SetBoss_State "NewEnumerator1")
  (bind _returnvalue (Game|SpawnActorfromClass "/Game/AProject/QueenOfHeart/QueenSkill/Blueprints/BP_Shield.BP_Shield_C" (Math|Transform|MakeTransform "-2900.000000,-360.000000,1215.000000" "0, 0, 0" "0.000000,0.000000,0.000000") "AlwaysSpawn" 0 0))
  (Variables|Default|SetShieldActor _returnvalue))

(event EventTick
  (params (DeltaSeconds :type Float%20%28single-precision%29))
  (switch Utilities|FlowControl|Switch|SwitchonBoss_Enum (Variables|Default|GetBoss_State)
    (:NewEnumerator0
      (Utilities|FlowControl|DoOnce false :!label _label
        (:Completed
          (CallFunction|Shield)
          (goto _label_2 Reset))))
    (:NewEnumerator1
      (CallFunction|Idle)
      (goto _label Reset))
    (:NewEnumerator2
      (CallFunction|Attack))
    (:NewEnumerator3
      (Utilities|FlowControl|DoOnce false :!label _label_2
        (:Completed
          (CallFunction|Rest))))
    (:NewEnumerator4
      (Utilities|FlowControl|DoOnce false
        (:Completed
          (CallFunction|Died))))))

(event Game|Damage|EventAnyDamage
  (params (Damage :type Float%20%28single-precision%29) (DamageType :type Damage%20Type%20Object%20Reference) (InstigatedBy :type Controller%20Object%20Reference) (DamageCauser :type Actor%20Object%20Reference))
  ;[0.02416 0 0 1 45] Damaged When Rest State
  (Utilities|FlowControl|DoOnce true
    (:Completed
      (bind _output_get (Variables|Default|SetHealth (- (Variables|Default|GetHealth) Damage)))
      (if (> _output_get 0.0)
        (Variables|Animate|Bool|SetbDamaged%20Ani true)
        (Utilities|FlowControl|Delay 0.4)
        (Variables|Animate|Bool|SetbDamaged%20Ani false)
        (Utilities|FlowControl|Delay 2.0)
        (Variables|Default|SetBoss_State "NewEnumerator0")
        (else
          (Variables|Default|SetBoss_State "NewEnumerator4"))))))

(fn ConstructionScript)

(fn WatchTarget)