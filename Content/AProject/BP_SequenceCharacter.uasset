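; BP_SequenceCharacter is a rabbit character that appears across six scripted sequences and drives tutorial beats between them.
; Start/end events for each sequence stop or resume its looping idle animation, some also snapping it to hardcoded transforms.
; After the second sequence, a delay and two chained one-shot audio components lead to BP_Hint's hint.
; Bow tutorial audio accompanies revealing BP_Picture, and FinTu audio destroys BP_Stop when finished.
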(event Custom|First%20Seq%20End
  (Transformation|SetActorLocationAndRotation "-2629.000000,-1269.000000,100.000000" "0,50.000000, 0")
  (Components|Animation|PlayAnimation (Variables|Default|GetSkeletalMesh) "/Game/KGW/rabbit/animations/rabbit_idle.rabbit_idle" true))

(event Custom|First%20Seq%20Start
  (Audio|Components|Audio|Stop (Variables|Default|GetSkeletalMesh)))

(event Custom|Forth%20Seq%20End
  (Components|Animation|PlayAnimation (Variables|Default|GetSkeletalMesh) "/Game/KGW/rabbit/animations/rabbit_idle.rabbit_idle" true))

(event Custom|Third%20Seq%20Start
  (Audio|Components|Audio|Stop (Variables|Default|GetSkeletalMesh)))

(event Custom|Third%20Seq%20End
  (Transformation|SetActorLocationAndRotation "-1089.000000,-1340.000000,396.000000" "0,45.000000, 0")
  (Components|Animation|PlayAnimation (Variables|Default|GetSkeletalMesh) "/Game/KGW/rabbit/animations/rabbit_idle.rabbit_idle" true))

(event Custom|Forth%20Seq%20Start
  (Audio|Components|Audio|Stop (Variables|Default|GetSkeletalMesh)))

(event Custom|Bow%20Tutorial
  (bind _returnvalue (AddComponent|AddAudioComponent false))
  (EventDispatchers|AssignOnAudioFinished _returnvalue (delegate Custom|CustomEvent))
  (bind _returnvalue_2 (Actor|GetActorOfClass "/Game/stylized_castle/meshes/interior_props/picture/BP_Picture.BP_Picture_C"))
  (Default|Visible _returnvalue_2))

(event Custom|AudioFinished1
  (Components|DestroyComponent (stale Custom|Second%20Seq%20End _returnvalue))
  (bind _returnvalue (AddComponent|AddAudioComponent false))
  (EventDispatchers|AssignOnAudioFinished _returnvalue (delegate Custom|Audio%20Finished2)))

(event Custom|Second%20Seq%20End
  (Components|Animation|PlayAnimation (Variables|Default|GetSkeletalMesh) "/Game/KGW/rabbit/animations/rabbit_idle.rabbit_idle" true)
  (Utilities|FlowControl|Delay 8.0)
  (bind _returnvalue (AddComponent|AddAudioComponent false))
  (EventDispatchers|AssignOnAudioFinished _returnvalue (delegate Custom|AudioFinished1)))

(event Custom|Audio%20Finished2
  (Components|DestroyComponent (stale Custom|AudioFinished1 _returnvalue))
  (bind _returnvalue (Actor|GetActorOfClass "/Game/AProject/Blueprints/BP_Hint.BP_Hint_C"))
  (Default|Hint _returnvalue))

(event Custom|Fin%20Tu
  (bind _returnvalue (AddComponent|AddAudioComponent false))
  (EventDispatchers|AssignOnAudioFinished _returnvalue (delegate Custom|CustomEvent_1)))

(event Custom|CustomEvent
  (Components|DestroyComponent (stale Custom|Bow%20Tutorial _returnvalue)))

(event Custom|Second%20Seq%20Start
  (Audio|Components|Audio|Stop (Variables|Default|GetSkeletalMesh)))

(event Custom|CustomEvent_1
  (Components|DestroyComponent (stale Custom|Fin%20Tu _returnvalue))
  (bind _returnvalue (Actor|GetActorOfClass "/Game/AProject/Blueprints/BP_Stop.BP_Stop_C"))
  (Actor|DestroyActor _returnvalue))

(event Custom|Fifth%20Seq%20Start
  (Transformation|SetActorLocationAndRotation "-1087.000000,-1352.000000,398.000000" "0,45.000000, 0")
  (Audio|Components|Audio|Stop (Variables|Default|GetSkeletalMesh)))

(event Custom|Hint%20Sound)

(event Custom|Fifth%20Seq%20End
  (Components|Animation|PlayAnimation (Variables|Default|GetSkeletalMesh) "/Game/KGW/rabbit/animations/rabbit_idle.rabbit_idle" true))

(event Custom|Sixth%20Seq%20Start
  (Audio|Components|Audio|Stop (Variables|Default|GetSkeletalMesh)))

(event Custom|Sixth%20Seq%20End
  (Components|Animation|PlayAnimation (Variables|Default|GetSkeletalMesh) "/Game/KGW/rabbit/animations/rabbit_idle.rabbit_idle" true))

(event EventBeginPlay
  (Components|Animation|PlayAnimation (Variables|Default|GetSkeletalMesh) "/Game/KGW/rabbit/animations/rabbit_idle.rabbit_idle" true))

(event EventTick
  (params (DeltaSeconds :type Float%20%28single-precision%29)))

(fn ConstructionScript)