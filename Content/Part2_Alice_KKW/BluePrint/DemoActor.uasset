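; DemoActor is a demo actor for Vosk speech recognition with push-to-talk recording and audio playback.
; On BeginPlay it binds partial and final result events, initializes Vosk against a local language server and starts voice capture.
; Pressing R begins capture, and releasing it finishes capture and plays the samples back as 16 kHz mono 2D sound.
; Recognized text goes to ProcessPartialResult and ProcessFinalResult, both empty stubs.
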(event Custom|PartialResultReceived
  (params (Text :type String))
  ;[1 1 1] Process realtime results
  (CallFunction|ProcessPartialResult Text))

(event Custom|FinalResultReceived
  (params (Text :type String))
  ;[1 1 1] Process final results
  (CallFunction|ProcessFinalResult Text))

(event EventBeginPlay
  (Utilities|FlowControl|Sequence
    (:then_0
      ;[1 1 1] Process realtime results
      (EventDispatchers|AssignOnPartialResultReceived (Variables|Default|GetVosk) (delegate Custom|PartialResultReceived)))
    (:then_1
      ;[1 1 1] Process final results
      (EventDispatchers|AssignOnFinalResultReceived (Variables|Default|GetVosk) (delegate Custom|FinalResultReceived)))
    (:then_2
      ;[1 1 1] Connect to language server
      (Class|VoskComponent|Initialize (Variables|Default|GetVosk) "localhost" 8080) ; Connect to server
      (Class|VoskComponent|BeginCapture (Variables|Default|GetVosk)) ; Start voice capture
    )))

(event Input|KeyboardEvents|R
  (params (Key :type Key%20Structure))
  (bind _vosk (Variables|Default|GetVosk))
  (:Pressed
    (Class|VoskComponent|BeginCapture _vosk))
  (:Released
    (bind _capturedata (Class|VoskComponent|FinishCapture _vosk))
    (bind _returnvalue (Class|VoskComponent|SamplestoSound _capturedata 16000 1))
    (Audio|PlaySound2D _returnvalue 1.0 1.0 0.0 0 0)))

(fn ConstructionScript)

(fn ProcessPartialResult
  (params (Value :type String)))

(fn ProcessFinalResult
  (params (Value :type String)))