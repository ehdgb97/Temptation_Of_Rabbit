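; BPVoskPassSoundWave is a Vosk speech recognition test Blueprint that passes sound wave data to an external ASR server and prints transcripts.
; BeginPlay launches the server process, then after a model-loading delay connects to localhost and begins capture, printing partial and final results.
; Releasing R decompresses a sound and sends it in packets, relying on matching sample rates.
; EndPlay uninitializes Vosk and kills the server process.
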(event Custom|OnPartialResultReceived_Event_0
  (params (Text :type String))
  ;[1 1 1] Process partial result
  (Development|PrintString Text))

(event Custom|OnFinalResultReceived_Event_0
  (params (Text :type String))
  ;[1 1 1] Process final result
  (Development|PrintString Text))

(event EventBeginPlay
  (Utilities|FlowControl|Sequence
    (:then_0
      ;[1 1 1] Start external language server process
      (bind _returnvalue (Class|VoskComponent|BuildServerParameters (Utilities|Struct|MakeVoskServerParameters "localhost" 8080 1 (Variables|Default|GetParams%20Sample%20Rate) 0 false (Variables|Default|GetPathToLanguageModel))))
      (bind _processhandle (Class|VoskComponent|CreateProcess (Variables|Default|GetPathToAsrServer) _returnvalue))
      (Variables|Default|SetServerProcessHandle _processhandle))
    (:then_1
      ;[1 1 1] Connect to server. Note that server will be able to recognize your voice only when it loads language data to the RAM, this is why we delay. But you still can connect right away, in this case recognition may be not accurate (until data is loaded to RAM)
      (Utilities|FlowControl|Delay 3.0)
      (Class|VoskComponent|Initialize (Variables|Default|GetVosk) "localhost" 8080)
      (Development|PrintString "Initialized")
      (Class|VoskComponent|BeginCapture (Variables|Default|GetVosk)))
    (:then_2
      ;[1 1 1] Process partial result
      (EventDispatchers|AssignOnPartialResultReceived (Variables|Default|GetVosk) (delegate Custom|OnPartialResultReceived_Event_0)))
    (:then_3
      ;[1 1 1] Process final result
      (EventDispatchers|AssignOnFinalResultReceived (Variables|Default|GetVosk) (delegate Custom|OnFinalResultReceived_Event_0)))))

(event EventEndPlay
  (params (EndPlayReason :type EEndPlayReason%20Enum :default "Destroyed"))
  ;[0.2656 0.2656 0.2656] Kill server process and uninitialize internal websocket
  (Class|VoskComponent|Uninitialize (Variables|Default|GetVosk))
  (Utilities|FlowControl|Delay 0.2)
  (Class|VoskComponent|KillProcess (Variables|Default|GetServerProcessHandle)))

(event Input|KeyboardEvents|R
  (params (Key :type Key%20Structure))
  ;[1 1 1] Pass sound wave data to language server
  (:Released
    (bind _rawsamples (|DecompressSound 0 false)
      (:Finished
        (bind _returnvalue (Class|VoskComponent|SendVoiceDatatoLanguageServer (Variables|Default|GetVosk) _rawsamples))
        (Development|PrintString (Utilities|String|ToString(Boolean) _returnvalue))))))

(fn ConstructionScript)