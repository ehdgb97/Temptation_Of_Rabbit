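; Push-to-talk speech-to-text Blueprint that uses Vosk to show recognized speech on the HUD while R serves as the talk key.
; BeginPlay launches a local ASR server process with a language model, connects Vosk to localhost and binds result events; EndPlay uninitializes Vosk and kills the process.
; Pressing R starts capture; releasing it requests the final result and shows the partial text until the final-result event delivers its text.
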(event Custom|OnPartialResultReceived
  (params (Text :type String))
  ;[0.461 0.631 1] Bind to partial result received event
)

(event Custom|OnFinalResultReceived_Event_0
  (params (Text :type String))
  ;[0.4891 1 0.4062 1 25] >>>>>  Use final result  <<<<<
  (Default|SetText (Variables|Default|GetHUD) (Utilities|Text|ToText(String) Text) true))

(event Custom|OnConnectedToServer_Event_0
  (Development|PrintString "CONNECTED TO SERVER"))

(event EventBeginPlay
  (Utilities|FlowControl|Sequence
    (:then_0
      ;[1 1 1] Start language server
      (bind (_success _returnvalue) (Class|VoskComponent|BuildServerParameters (Utilities|Struct|MakeVoskServerParameters "localhost" 8080 1 16000 0 false (Variables|Default|GetPathToLanguageModel))))
      (if _success
        ;;[0.08235 1 0] !!! PATH TO asr_server_exe !!!
        ;;
        ;; Use this nodes:
        (bind _processhandle (Class|VoskComponent|CreateProcess (Variables|Default|GetAsrServerPath) _returnvalue false false))
        (Variables|Default|SetProcess%20Id _processhandle)))
    (:then_1
      ;[0.461 0.631 1] Bind to partial result received event
      (EventDispatchers|AssignOnPartialResultReceived (Variables|Default|GetVosk) (delegate Custom|OnPartialResultReceived))
      ;[0.4891 1 0.4062 1 25] >>>>>  Use final result  <<<<<
      (EventDispatchers|AssignOnFinalResultReceived (Variables|Default|GetVosk) (delegate Custom|OnFinalResultReceived_Event_0)))
    (:then_2
      (EventDispatchers|AssignOnConnectedtoServer (Variables|Default|GetVosk) (delegate Custom|OnConnectedToServer_Event_0)))
    (:then_3
      ;[0.4869 0.9502 1] Get reference to HUD
      (Utilities|FlowControl|Delay 0.2)
      (bind _asnew_hud (Utilities|Casting|CastToNewHUD (HUD|GetHUD (Game|GetPlayerController 0))))
      (Variables|/Game/Part2_Alice_KKW/BluePrint/NewHUD.NewHUD_C|SetHUDInstance _asnew_hud (Default|GetHudInstance _asnew_hud)))
    (:then_4
      (Class|VoskComponent|Initialize (Variables|Default|GetVosk) "localhost" 8080) ; Connect once
    )))

(event EventEndPlay
  (params (EndPlayReason :type EEndPlayReason%20Enum :default "Destroyed"))
  ;[0.08235 1 0] Shutdown server
  (Class|VoskComponent|Uninitialize (Variables|Default|GetVosk))
  (Class|VoskComponent|KillProcess (Variables|Default|GetProcess%20Id)))

(event Input|KeyboardEvents|R
  (params (Key :type Key%20Structure))
  (:Pressed
    (Class|VoskComponent|BeginCapture (Variables|Default|GetVosk))
    (Class|VoskComponent|ResetPartialResult (Variables|Default|GetVosk))
    (Class|VoskComponent|ResetFinalResult (Variables|Default|GetVosk))
    (Default|SetIsReady (Variables|Default|GetHUD) true))
  (:Released
    ;[1 0.6266 0.9991] Ask server for final result
    (Class|VoskComponent|RequestFinalResult (Variables|Default|GetVosk))
    (Class|VoskComponent|ResetRecognizer (Variables|Default|GetVosk))
    ;[0.8488 1 0.4769] >>>> Use partial (intermediate) result <<<<<
    (bind _hud (Variables|Default|GetHUD)
      (:then
        (Default|SetText _hud (Utilities|Text|ToText(String) (Class|VoskComponent|GetPartialResult (Variables|Default|GetVosk))) false))
      (:else
        _))
    (Default|SetIsReady (Variables|Default|GetHUD) false)))

(fn ConstructionScript)