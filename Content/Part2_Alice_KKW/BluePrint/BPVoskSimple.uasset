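; Voice-controlled actor that uses a Vosk speech server on localhost to move itself or show replies on a text render.
; Holding R connects and captures voice; releasing requests the final result, processes the current partial text, then disconnects.
; Keyword-array substring matches select a directional step, name reply or abilities reply.
; Vosk events feed connection state and partial or final transcripts to the HUD; Escape quits.
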(event Custom|OnPartialResultReceived_Event_0
  (params (Text :type String))
  ;[0 0 0] Events binding
  ;;[1 1 1] Use partial result (부분적인 결과를 사용)
  (bind _hudinstance (Variables|Default|GetHUDInstance)
    (:then
      (Default|SetText _hudinstance (Utilities|Text|ToText(String) Text) false))
    (:else)))

(event Custom|OnFinalResultReceived_Event_0
  (params (Text :type String))
  ;[0 0 0] Events binding
  ;;[1 1 1] Use final result (마지막 결과창)
  (Default|SetText (Variables|Default|GetHUDInstance) (Utilities|Text|ToText(String) Text) true))

(event Custom|OnConnectedToServer_Event_0
  ;[0 0 0] Events binding
  ;;[1 1 1] When connected to server (우리가 서버에 연결)
  (bind _hudinstance (Variables|Default|GetHUDInstance)
    (:then
      (Default|SetIsReady _hudinstance true))
    (:else)))

(event Custom|OnConnectionTerminated_Event_0
  (params (StatusCode :type Integer) (Reason :type String) (WasClean :type Boolean))
  ;[0 0 0] Events binding
  ;;[1 1 1] When disconnected (우리가 서버에 연결해제)
  (bind _hudinstance (Variables|Default|GetHUDInstance)
    (:then
      (Default|SetIsReady _hudinstance false))
    (:else)))

(event EventBeginPlay
  (Utilities|FlowControl|Sequence
    (:then_0
      ;[0 0 0] Events binding
      ;;[1 1 1] When connected to server (우리가 서버에 연결)
      (EventDispatchers|AssignOnConnectedtoServer (Variables|Default|GetVosk) (delegate Custom|OnConnectedToServer_Event_0)))
    (:then_1
      ;;[1 1 1] When disconnected (우리가 서버에 연결해제)
      (EventDispatchers|AssignOnConnectionTerminated (Variables|Default|GetVosk) (delegate Custom|OnConnectionTerminated_Event_0)))
    (:then_2
      ;;[1 1 1] Use partial result (부분적인 결과를 사용)
      (EventDispatchers|AssignOnPartialResultReceived (Variables|Default|GetVosk) (delegate Custom|OnPartialResultReceived_Event_0)))
    (:then_3
      ;;[1 1 1] Use final result (마지막 결과창)
      (EventDispatchers|AssignOnFinalResultReceived (Variables|Default|GetVosk) (delegate Custom|OnFinalResultReceived_Event_0)))
    (:then_4
      ;;[1 1 1] HUD setup
      (Utilities|FlowControl|Delay 1.0)
      (bind _asnew_hud (Utilities|Casting|CastToNewHUD (HUD|GetHUD (Game|GetPlayerController 0))))
      (Variables|/Game/Part2_Alice_KKW/BluePrint/NewHUD.NewHUD_C|SetHUDInstance _asnew_hud (Default|GetHudInstance _asnew_hud)))))

(event EventEndPlay
  (params (EndPlayReason :type EEndPlayReason%20Enum :default "Destroyed")))

(event Input|KeyboardEvents|R
  (params (Key :type Key%20Structure))
  ;[0.3405 0.9219 0.09603] Connect -> start capture -> disconnect -> end capture
  (:Pressed
    (Class|VoskComponent|Initialize (Variables|Default|GetVosk) "localhost" 8080) ; Connect to server (서버 ui에 있는 모든 항목에 연결)
    (Class|VoskComponent|BeginCapture (Variables|Default|GetVosk)) ; Start voice capture 클라이언트가 연결되면 음성 캡쳐를 시작
    ;;[0.4419 0.3749 1] Reset internal result variables
    (Class|VoskComponent|ResetFinalResult (Variables|Default|GetVosk))
    (Class|VoskComponent|ResetPartialResult (Variables|Default|GetVosk)))
  (:Released
    ;;[1 1 1] 서버에 메세지를 보내는 것을 종료 시키고 최종 결과를 보낸다
    (Class|VoskComponent|RequestFinalResult (Variables|Default|GetVosk)) ; Right before shutting down - ask server to send final result.\nThis will send special message to server.\n\nDefault message - {"eof" : 1}\n\nTo override message, use - "Set Final Result Request Message".\n\nNOTE: This is needed only if you change server code
    (CallFunction|ProcessFinalResult (Class|VoskComponent|GetPartialResult (Variables|Default|GetVosk)))
    (Utilities|FlowControl|Delay 0.5)
    ;;[1 1 1] 로컷 소켓을 초기화 하고 이후 서버에 연결종료
    (Class|VoskComponent|Uninitialize (Variables|Default|GetVosk)) ; This will close socket (client)
    (Class|VoskComponent|FinishCapture (Variables|Default|GetVosk)) ; Shut down voice capture
    (if (not (Class|VoskComponent|IsInitialized (Variables|Default|GetVosk)))
      (Development|PrintString "SERVER IS NOT CONNECTED" true true "(R=1.000000,G=0.127780,B=0.000000,A=1.000000)" 5.0))))

(event Input|KeyboardEvents|Escape
  (params (Key :type Key%20Structure))
  (:Released
    (Game|QuitGame 0 "Quit" false)))

(fn ConstructionScript)

(fn ProcessFinalResult
  (params (Result :type String))
  (bind _output_get (LocalVariables|SetSourceText Result))
  ;[1 1 1] forward
  (if (CallFunction|StringHasTags _output_get (LocalVariables|GetForwardKeywords))
    (Transformation|AddActorLocalOffset (* (Transformation|GetActorForwardVector) (* (Variables|Default|GetStepSize) -1.0)) false false)
    (else
      ;[1 1 1] backward
      (if (CallFunction|StringHasTags (LocalVariables|GetSourceText) (LocalVariables|GetBackwardKeywords))
        (Transformation|AddActorLocalOffset (* (Transformation|GetActorForwardVector) (Variables|Default|GetStepSize)) false false)
        (else
          ;[1 1 1] left
          (if (CallFunction|StringHasTags (LocalVariables|GetSourceText) (LocalVariables|GetLeftKeywords))
            (Transformation|AddActorLocalOffset (* (Transformation|GetActorRightVector) (Variables|Default|GetStepSize)) false false)
            (else
              ;[1 1 1] right
              (if (CallFunction|StringHasTags (LocalVariables|GetSourceText) (LocalVariables|GetRightKeywords))
                (Transformation|AddActorLocalOffset (* (Transformation|GetActorRightVector) (* (Variables|Default|GetStepSize) -1.0)) false false)
                (elif (CallFunction|StringHasTags (LocalVariables|GetSourceText) (LocalVariables|GetIdentifyYourselfKeywords))
                  (Rendering|Components|TextRender|SetText (Variables|Default|GetTextRender) (Utilities|Text|MakeLiteralText "My name is \"Cube\", hello!"))
                  (elif (CallFunction|StringHasTags (LocalVariables|GetSourceText) (LocalVariables|GetWhatCanYouDo))
                    (Rendering|Components|TextRender|SetText (Variables|Default|GetTextRender) (Utilities|Text|MakeLiteralText "* I can tell you my name 
* I can move (forward, backward, left and right)"))))))))))))

(fn StringHasTags
  (params (SrcString :type String) (Tags :type Array%20of%20Strings))
  (LocalVariables|SetSrcStr SrcString)
  (bind _array_element (Utilities|Array|ForEachLoopwithBreak Tags :!label _label)
    (:LoopBody
      (if (Utilities|String|Contains (LocalVariables|GetSrcStr) _array_element)
        (LocalVariables|Setfound true)
        (goto _label Break)))
    (:Completed
      (return (LocalVariables|Getfound)))))