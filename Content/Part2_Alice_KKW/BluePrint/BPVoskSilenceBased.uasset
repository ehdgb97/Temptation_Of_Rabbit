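; Voice input Blueprint that runs offline Vosk speech recognition and detects when the player stops talking, without requiring any key press.
; On BeginPlay it launches a local ASR server process, connects and starts capture; EndPlay shuts these down.
; Non-empty partial results restart a retriggerable delay whose expiry signals silence and resets the recognizer.
; Recognized text goes to the HUD, and Tick copies the talking flag to the game state and HUD.
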(event Custom|OnPartialResultReceived_Event_0
  (params (Text :type String))
  (Utilities|FlowControl|Sequence
    (:then_0
      (if (not (Utilities|Array|IsEmpty Text))
        (Variables|Default|SetIs%20Talking true)
        ;[0.1719 1 0] This duration controls sensitivity of stop talking detection. Set it to 1s or greater, to give server chance to process your voice
        (Utilities|FlowControl|RetriggerableDelay 0.33)
        (Variables|Default|SetIs%20Talking false)
        (CallFunction|OnStoppedTalking)))
    (:then_1
      (Default|SetText (Variables|Default|GetHUD) (Utilities|Text|ToText(String) Text) false))))

(event Custom|OnFinalResultReceived_Event_0
  (params (Text :type String))
  ;[0.05208 0.05208 0.05208] Set final result to final result widget
  (Default|SetText (Variables|Default|GetHUD) (Utilities|Text|ToText(String) Text) true))

(event Custom|OnStoppedTalking
  (Class|VoskComponent|ResetRecognizer (Variables|Default|GetVosk))
  (Variables|Default|SetIs%20Talking false)
  (Utilities|FlowControl|Sequence
    (:then_0
      ;[1 1 1] Display cumulative phrase in partial result widget
      (Default|SetText (Variables|Default|GetHUD) (Utilities|Text|ToText(String) (Variables|Default|GetPartialResult)) false))
    (:then_1
      ;[0.1306 1 0] Cut cumulative phrase by special word, and take right hand side. Display phrase in final result widget
      ;
      ; e.g. "ok robot, are you gonna to enslave humanity?" -> ", are you gonna to enslave humanity?"
      (Default|SetText (Variables|Default|GetHUD) (Utilities|Text|ToText(String) (Class|VoskComponent|GetPartialResult (Variables|Default|GetVosk))) false))))

(event EventBeginPlay
  ;[0.3265 0.3458 1 1 30] This example demonstrates how to NOT require any input from user
  (Utilities|FlowControl|Sequence
    (:then_0
      (bind (_success _returnvalue) (Class|VoskComponent|BuildServerParameters (Utilities|Struct|MakeVoskServerParameters "localhost" 8080 1 16000 0 false (Variables|Default|GetPathToLanguageModel))))
      (if _success
        (bind _processhandle (Class|VoskComponent|CreateProcess (Variables|Default|GetAsrSereverPath) _returnvalue false false))
        (Variables|Default|SetServerProcessHandle _processhandle)))
    (:then_1
      ;[0.05208 0.05208 0.05208] Set final result to final result widget
      (EventDispatchers|AssignOnFinalResultReceived (Variables|Default|GetVosk) (delegate Custom|OnFinalResultReceived_Event_0)))
    (:then_2
      (EventDispatchers|AssignOnPartialResultReceived (Variables|Default|GetVosk) (delegate Custom|OnPartialResultReceived_Event_0)))
    (:then_3
      (Class|VoskComponent|Initialize (Variables|Default|GetVosk) "localhost" 8080)
      (Class|VoskComponent|BeginCapture (Variables|Default|GetVosk)))
    (:then_4
      (Utilities|FlowControl|Delay 0.2)
      (bind _asnew_hud (Utilities|Casting|CastToNewHUD (HUD|GetHUD (Game|GetPlayerController 0))))
      (Variables|/Game/Part2_Alice_KKW/BluePrint/NewHUD.NewHUD_C|SetHUDInstance _asnew_hud (Default|GetHudInstance _asnew_hud)))))

(event EventTick
  (params (DeltaSeconds :type Float%20%28single-precision%29))
  (Utilities|FlowControl|Delay 0.2)
  (bind _asnew_game_state_base (Utilities|Casting|CastToNewGameStateBase (Game|GetGameState)))
  (bind _output_get (Variables|/Game/Part2_Alice_KKW/BluePrint/NewGameStateBase.NewGameStateBase_C|SetIs%20Talking _asnew_game_state_base (Variables|Default|GetIs%20Talking)))
  (Default|SetIsReady (Variables|Default|GetHUD) _output_get))

(event EventEndPlay
  (params (EndPlayReason :type EEndPlayReason%20Enum :default "Destroyed"))
  ;[1 1 1] Shutdown connection and voice capture
  (Class|VoskComponent|Uninitialize (Variables|Default|GetVosk))
  (Class|VoskComponent|FinishCapture (Variables|Default|GetVosk))
  (Class|VoskComponent|KillProcess (Variables|Default|GetServerProcessHandle)))

(fn ConstructionScript)

(fn CutPhrase
  (params (Phrase :type String) (Separator :type String))
  (bind (_lefts _rights _returnvalue) (Utilities|String|Split Phrase Separator "IgnoreCase" "FromEnd"))
  (return (select _returnvalue _rights Phrase)))

(fn NewFunction0)