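; BP_PostProcess is an actor that switches a post-process effect according to rose progress in the maze puzzle.
; When its Box is overlapped, it casts its owner to BP_MazePuzzle and makes the PostProcess component visible.
; Blend weight snaps off if the puzzle's BloomRoseCount equals ten, otherwise to full.
; The ChangeBW timeline is unreachable, so no fade occurs.
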(event OnComponentBeginOverlap(Box)
  (params (OverlappedComponent :type Primitive%20Component%20Object%20Reference) (OtherActor :type Actor%20Object%20Reference) (OtherComp :type Primitive%20Component%20Object%20Reference) (OtherBodyIndex :type Integer) (bFromSweep :type Boolean) (SweepResult :type Hit%20Result%20Structure%20%28by%20ref%29))
  (bind _postprocess (Variables|Default|GetPostProcess))
  (bind _asbp_maze_puzzle (Utilities|Casting|CastToBP_MazePuzzle (Components|GetOwner)))
  (Rendering|SetVisibility (Variables|Default|GetPostProcess) true false)
  (if (== (Variables|/Game/AKJK/MazeGarden/BP_MazePuzzle.BP_MazePuzzle_C|GetbloomRoseCount _asbp_maze_puzzle) 10)
    (Variables|/Script/Engine.PostProcessComponent|SetBlendWeight _postprocess 0.0)
    (else
      (Variables|/Script/Engine.PostProcessComponent|SetBlendWeight _postprocess 1.0))))

(event OnComponentDeactivated(PostProcess)
  (params (Component :type Actor%20Component%20Object%20Reference)))

(event EventBeginPlay)

(event Collision|EventActorBeginOverlap
  (params (OtherActor :type Actor%20Object%20Reference)))

(fn ConstructionScript)