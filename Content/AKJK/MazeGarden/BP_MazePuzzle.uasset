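; Maze garden puzzle that opens the maze exit once the player has painted enough roses red.
; BloomRose counts roses; at the threshold it triggers Exit once, teleports Alice in front of the exit behind camera fades, then removes the paintbrush and adds audio.
; Exit waits briefly, then plays an earthquake sound while a timeline slides the maze mesh aside, with a one-off leaf burst.
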(event Custom|Exit
  (params (isRoseRed :type Boolean))
  ;[1 1 1] 빨간장미 10개 이상일 때 미로퍼즐이 왼쪽으로 이동하면서 효과음내기
  (Utilities|FlowControl|Delay 2.0)
  (Utilities|FlowControl|DoOnce false
    (:Completed
      (Audio|SpawnSound2D "/Game/AKJK/Sound/Earthquake/ES_Earthquake_Debris_18_-_SFX_Producer.ES_Earthquake_Debris_18_-_SFX_Producer" 1.0 1.0 0.0 0)
      (bind _newtrack_0 (Timeline|Timeline_0 Play)
        (:Update
          (Transformation|SetRelativeTransform (Variables|Default|GetSMM_MazePuzzle_2) (Math|Transform|MakeTransform (Math|Vector|MakeVector (- 1367.523438 _newtrack_0) 573.391724 287.296814) "0, 0, 0" "1,1,1") false false)
          (Utilities|FlowControl|DoOnce false
            (:Completed
              (Effects|SpawnEmitteratLocation "/Game/AKJK/Particle/P_Leaves.P_Leaves" "0, 0, 0"))))))))

(event Custom|BloomRose
  ;[1 1 1] 장미 10송이 이상일 때 열려라 참깨!
  (bind _output_get (Variables|Default|SetbloomRoseCount (+ (Variables|Default|GetbloomRoseCount) 1)))
  (if (>= _output_get (Variables|Default|GetHaveToPaint))
    (Utilities|FlowControl|DoOnce false
      (:Completed
        (CallFunction|Exit false)
        ;[1 1 1] 장미 다 칠해지면 미로출구 앞으로 이동
        (bind _asalice_player (Utilities|Casting|CastToAlicePlayer (Game|Player|GetPlayerPawn 0)))
        (CameraFades|StartCameraFade :self (Game|GetPlayerCameraManager 0) :ToAlpha 1.0 :Duration 1.0 :bHoldWhenFinished true)
        (Utilities|FlowControl|Delay 1.0)
        (Transformation|SetActorLocationAndRotation _asalice_player (Math|Vector|MakeVector 1665.0 920.355042 97.198059) (Math|Rotator|MakeRotator 0.0 0.0 -9e+01))
        (CameraFades|StartCameraFade :self (Game|GetPlayerCameraManager 0) :FromAlpha 1.0 :Duration 1.0 :bHoldWhenFinished true)
        (Utilities|FlowControl|Delay 1.0)
        (bind _returnvalue (Actor|GetActorOfClass "/Game/AKJK/BluePrint/BP_PaintBrush.BP_PaintBrush_C"))
        (Utilities|FlowControl|DoOnce false
          (:Completed
            (Default|Disappear _returnvalue)
            (AddComponent|AddAudioComponent false)))))))

(fn ConstructionScript)