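; Mini door for the maze garden that swings open when AlicePlayer enters its Box trigger and closes after the player leaves.
; The Door_anim timeline scales its track by Angle to set the Door's yaw, and reverses one second after the overlap ends.
; A DoOnce on the timeline update plays a spooky creak as a 2D sound only the first time the door moves, as it is never reset.
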(event OnComponentBeginOverlap(Box)
  (params (OverlappedComponent :type Primitive%20Component%20Object%20Reference) (OtherActor :type Actor%20Object%20Reference) (OtherComp :type Primitive%20Component%20Object%20Reference) (OtherBodyIndex :type Integer) (bFromSweep :type Boolean) (SweepResult :type Hit%20Result%20Structure%20%28by%20ref%29))
  (Utilities|Casting|CastToAlicePlayer OtherActor)
  (bind _newtrack_0 (Timeline|door_anim Play)
    (:Update
      (Transformation|SetRelativeRotation (Variables|Default|GetDoor) (Math|Rotator|MakeRotator 0.0 0.0 (* _newtrack_0 (Variables|Default|GetAngle))) false false)
      (Utilities|FlowControl|DoOnce false
        (:Completed
          (Audio|SpawnSound2D "/Game/AKJK/Sound/DoorOpen/Creaking_Door_Spooky_Sound.Creaking_Door_Spooky_Sound" 1.0 1.0 0.0 0))))))

(event OnComponentEndOverlap(Box)
  (params (OverlappedComponent :type Primitive%20Component%20Object%20Reference) (OtherActor :type Actor%20Object%20Reference) (OtherComp :type Primitive%20Component%20Object%20Reference) (OtherBodyIndex :type Integer))
  (Utilities|Casting|CastToAlicePlayer OtherActor)
  (Utilities|FlowControl|Delay 1.0)
  (bind _newtrack_0 (Timeline|door_anim Reverse)
    (:Update
      (Transformation|SetRelativeRotation (Variables|Default|GetDoor) (Math|Rotator|MakeRotator 0.0 0.0 (* _newtrack_0 (Variables|Default|GetAngle))) false false)
      (Utilities|FlowControl|DoOnce false
        (:Completed
          (Audio|SpawnSound2D "/Game/AKJK/Sound/DoorOpen/Creaking_Door_Spooky_Sound.Creaking_Door_Spooky_Sound" 1.0 1.0 0.0 0))))))

(fn ConstructionScript)