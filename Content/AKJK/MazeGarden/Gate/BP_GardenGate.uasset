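; Maze garden double gate that swings both leaves when the player (AlicePlayer) enters its box trigger.
; Begin overlap passes a DoOnce with no reset, plays a 2D heavy gate closing sound and starts two timelines that scale the Angle90 variable into each leaf's relative yaw.
; End overlap waits briefly, then reverses both timelines, so the forward swing and sound happen only on the first entry.
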(event OnComponentBeginOverlap(Box)
  (params (OverlappedComponent :type Primitive%20Component%20Object%20Reference) (OtherActor :type Actor%20Object%20Reference) (OtherComp :type Primitive%20Component%20Object%20Reference) (OtherBodyIndex :type Integer) (bFromSweep :type Boolean) (SweepResult :type Hit%20Result%20Structure%20%28by%20ref%29))
  (Utilities|Casting|CastToAlicePlayer OtherActor)
  (Utilities|FlowControl|DoOnce false
    (:Completed
      (Audio|SpawnSound2D "/Game/AKJK/Sound/DoorOpen/Heavy_Gate_Closing.Heavy_Gate_Closing" 1.0 1.0 0.0 0)
      (Utilities|FlowControl|Sequence
        (:then_0
          (bind _newtrack_0 (Timeline|Gate Play)
            (:Update
              (Transformation|SetRelativeRotation (Variables|Default|GetSM%20Gate_R) (Math|Rotator|MakeRotator 0.0 0.0 (* _newtrack_0 (Variables|Default|Getangle%2090))) false false))))
        (:then_1
          (bind _newtrack_0_2 (Timeline|Timeline_0 Play)
            (:Update
              (Transformation|SetRelativeRotation (Variables|Default|GetSM%20Gate_L) (Math|Rotator|MakeRotator 0.0 0.0 (* _newtrack_0_2 (Variables|Default|Getangle%20-90))) false false))))))))

(event OnComponentEndOverlap(Box)
  (params (OverlappedComponent :type Primitive%20Component%20Object%20Reference) (OtherActor :type Actor%20Object%20Reference) (OtherComp :type Primitive%20Component%20Object%20Reference) (OtherBodyIndex :type Integer))
  (Utilities|Casting|CastToAlicePlayer OtherActor)
  (Utilities|FlowControl|Delay 1.5)
  (Utilities|FlowControl|Sequence
    (:then_0
      (bind _newtrack_0 (Timeline|Gate Reverse)
        (:Update
          (Transformation|SetRelativeRotation (Variables|Default|GetSM%20Gate_R) (Math|Rotator|MakeRotator 0.0 0.0 (* _newtrack_0 (Variables|Default|Getangle%2090))) false false))))
    (:then_1
      (bind _newtrack_0_2 (Timeline|Timeline_0 Reverse)
        (:Update
          (Transformation|SetRelativeRotation (Variables|Default|GetSM%20Gate_L) (Math|Rotator|MakeRotator 0.0 0.0 (* _newtrack_0_2 (Variables|Default|Getangle%20-90))) false false))))))

(event EventBeginPlay)

(event Collision|EventActorBeginOverlap
  (params (OtherActor :type Actor%20Object%20Reference)))

(event EventTick
  (params (DeltaSeconds :type Float%20%28single-precision%29)))

(fn ConstructionScript)