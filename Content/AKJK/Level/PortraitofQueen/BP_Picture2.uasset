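; BP_Picture2 is a picture actor in the PortraitofQueen level that drops when a BP_Arrow first overlaps its box.
; The hit hides the outline mesh and plays a timeline driving the actor's location and rotation, with two delayed drop sounds.
; When the timeline finishes, it calls FinTu on BP_SequenceCharacter.
; A separate Visible event shows the outline with a dynamic M_outline material, setting its color and scale.
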(event OnComponentBeginOverlap(Box)
  (params (OverlappedComponent :type Primitive%20Component%20Object%20Reference) (OtherActor :type Actor%20Object%20Reference) (OtherComp :type Primitive%20Component%20Object%20Reference) (OtherBodyIndex :type Integer) (bFromSweep :type Boolean) (SweepResult :type Hit%20Result%20Structure%20%28by%20ref%29))
  (Utilities|Casting|CastToBP_Arrow OtherActor)
  (Utilities|FlowControl|DoOnce false
    (:Completed
      (Rendering|SetVisibility (Variables|Default|GetUI%20Outline) false false)
      (bind (_direction _새_트랙_0 _새_트랙_1) (Timeline|타임라인_0 PlayFromStart)
        (:Update
          (Transformation|SetActorLocationAndRotation _새_트랙_0 (Math|Rotator|MakeRotator (.x _새_트랙_1) (.y _새_트랙_1) (.z _새_트랙_1)))
          (Utilities|FlowControl|DoOnce false
            (:Completed
              (Utilities|FlowControl|Delay 0.4)
              (Audio|SpawnSound2D "/Game/AProject/BGM/Drop.Drop" 1.0 1.0 0.0 0)
              (Utilities|FlowControl|Delay 0.55)
              (Audio|SpawnSound2D "/Game/AProject/BGM/Drop.Drop" 1.0 1.0 0.0 0))))
        (:Finished
          (bind _returnvalue (Actor|GetActorOfClass "/Game/AProject/BP_SequenceCharacter.BP_SequenceCharacter_C"))
          (Default|FinTu _returnvalue))))))

(event Custom|Visible
  (bind _ui_outline (Variables|Default|GetUI%20Outline))
  (Rendering|SetVisibility _ui_outline true false)
  (Rendering|Material|SetMaterial _ui_outline 0 0)
  (bind _returnvalue (Rendering|Material|CreateDynamicMaterialInstance _ui_outline 0 "/Game/AKJK/PaintingMaterials/M_outline.M_outline" "None" :!class /Script/Engine.PrimitiveComponent))
  (bind _output_get (Variables|Default|SetNewVar_0 _returnvalue))
  (Rendering|Material|SetVectorParameterValue _output_get "Color" (Variables|Default|GetValue) :!class /Script/Engine.MaterialInstanceDynamic)
  (Rendering|Material|SetScalarParameterValue _output_get "Scale" 0.75 :!class /Script/Engine.MaterialInstanceDynamic))

(event EventBeginPlay)

(event Collision|EventActorBeginOverlap
  (params (OtherActor :type Actor%20Object%20Reference)))

(event EventTick
  (params (DeltaSeconds :type Float%20%28single-precision%29)))

(fn ConstructionScript)