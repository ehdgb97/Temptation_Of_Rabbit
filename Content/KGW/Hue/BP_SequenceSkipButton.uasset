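; BP_SequenceSkipButton is an actor that floats near the AlicePlayer camera; the skip action itself is not in its graphs.
; BeginPlay caches the player, and Tick targets a point 100 units from the camera, blending flattened forward, right and down directions.
; Each frame it lerps toward that point by a fixed alpha, giving a frame-rate-dependent lazy follow, and turns on yaw only to face the camera.
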(event EventBeginPlay
  (bind _returnvalue (Actor|GetActorOfClass "/Game/KGW/VRTemplate/Blueprints/AlicePlayer.AlicePlayer_C"))
  (Variables|Default|SetAlice _returnvalue))

(event Collision|EventActorBeginOverlap
  (params (OtherActor :type Actor%20Object%20Reference)))

(event EventTick
  (params (DeltaSeconds :type Float%20%28single-precision%29))
  (bind _returnvalue (Transformation|GetActorLocation))
  (bind _alice (Variables|Default|GetAlice))
  (bind _camera (Variables|/Game/KGW/VRTemplate/Blueprints/AlicePlayer.AlicePlayer_C|GetCamera _alice))
  (bind _returnvalue_2 (Math|Vector|GetForwardVector _camera))
  (bind _returnvalue_3 (Transformation|GetWorldLocation _camera))
  (bind _returnvalue_4 (- _returnvalue_3 _returnvalue))
  (Transformation|SetActorLocationAndRotation (Math|Vector|Lerp(Vector) (Transformation|GetActorLocation) (+ (* (Math|Vector|Normalize (+ (* (Math|Vector|Normalize (+ (* (Math|Vector|Normalize (Math|Vector|MakeVector (.x _returnvalue_2) (.y _returnvalue_2) 0.0)) 2.5) (Math|Vector|GetRightVector _camera))) 1.5) (Math|Vector|VectorDown))) 1e+02) _returnvalue_3) 0.2) (Math|Conversions|RotationFromXVector (Math|Vector|Normalize (Math|Vector|MakeVector (.x _returnvalue_4) (.y _returnvalue_4) 0.0)))))

(fn ConstructionScript)